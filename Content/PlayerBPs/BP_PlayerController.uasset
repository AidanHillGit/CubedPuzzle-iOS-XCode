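; Player controller for the block puzzle game, managing the begin screen or tutorial, play HUD and end-of-level sequence.
; BeginPlay builds dynamic block and outline materials from saved color preferences, refreshing thumbnails in multi-color mode.
; AddWidgetToGame binds the HUD to a board or fill board, with CanSwitch polling before revealing the board HUD.
; Game over computes stars, pans the camera, then recursively flashes each piece before animating stars.
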(event Custom|AddWidgetToGame
  (params (BoardRef :type BP%20Board%20Manager%20Object%20Reference) (FillBoardRef :type BP%20Fill%20the%20Cube%20Board%20Object%20Reference))
  ;[0.15 0.15 0.15 0.5] Create The Players Play Game HUD Based On Game Mode
  (Utilities|IsValid BoardRef
    (:Is%20Valid
      (Utilities|FlowControl|DelayUntilNextTick)
      (bind _returnvalue (UserInterface|CreateWidget "/Game/PlayerBPs/PlayerHUD/WBP_HUDController.WBP_HUDController_C" self))
      (Widget|SetVisibility _returnvalue "Hidden")
      (Variables|Default|SetHUDControllerRef _returnvalue)
      (Variables|/Game/PlayerBPs/PlayerHUD/WBP_PlayGameHUD.WBP_PlayGameHUD_C|SetBoardRef (Variables|/Game/PlayerBPs/PlayerHUD/WBP_HUDController.WBP_HUDController_C|GetWBP_PlayGameHUD _returnvalue) BoardRef)
      (UserInterface|Viewport|AddtoViewport _returnvalue 0)
      (Variables|Default|SetHUDRef (Variables|/Game/PlayerBPs/PlayerHUD/WBP_HUDController.WBP_HUDController_C|GetWBP_PlayGameHUD _returnvalue))
      (Variables|Default|SetWidgetReady true)
      (CallFunction|CanSwitch)
      (if (Variables|Default|GetTutorialActive)
        (Default|SetTutorial (Variables|/Game/PlayerBPs/PlayerHUD/WBP_HUDController.WBP_HUDController_C|GetWBP_PlayGameHUD (Variables|Default|GetHUDControllerRef)))
        (Widget|SetVisibility (Variables|Default|GetHUDControllerRef) "Hidden")
        (Default|PlayTutorialOne (Variables|Default|GetTutorialWidget))))
    (:Is%20Not%20Valid
      (Utilities|FlowControl|DelayUntilNextTick)
      (bind _returnvalue_2 (UserInterface|CreateWidget "/Game/PlayerBPs/PlayerHUD/WBP_HUDController.WBP_HUDController_C" self))
      (Variables|Default|SetHUDControllerRef _returnvalue_2)
      (Variables|/Game/PlayerBPs/PlayerHUD/WBP_PlayGameHUD.WBP_PlayGameHUD_C|SetFillBoardRef (Variables|/Game/PlayerBPs/PlayerHUD/WBP_HUDController.WBP_HUDController_C|GetWBP_PlayGameHUD _returnvalue_2) FillBoardRef)
      (UserInterface|Viewport|AddtoViewport _returnvalue_2 0)
      (Variables|Default|SetHUDRef (Variables|/Game/PlayerBPs/PlayerHUD/WBP_HUDController.WBP_HUDController_C|GetWBP_PlayGameHUD _returnvalue_2))
      (Variables|Default|SetWidgetReady true))))

(event Custom|SetUpGameOverWidget
  (params (LevelName :type Name) (Moves :type Integer) (TimeTaken :type Float%20%28double-precision%29))
  (bind _totalstars (Default|StarsEarned (Variables|Default|GetSaveGameRef) LevelName Moves TimeTaken))
  (Widget|RemovefromParent (Variables|Default|GetHUDRef))
  (bind _returnvalue (UserInterface|CreateWidget "/Game/PlayerBPs/PlayerHUD/WBP_EndGame.WBP_EndGame_C"))
  (Variables|Default|SetEndGameRef _returnvalue)
  (UserInterface|Viewport|AddtoViewport _returnvalue 0)
  (Class|BPICallEndGame|OnGameOver(Message) _returnvalue true TimeTaken Moves _totalstars LevelName)
  (CallFunction|SmoothCameraRot))

(event Custom|GetDynamicMaterial
  (Utilities|Map|Clear (Variables|Default|GetIDtoMaterialMap))
  (bind _asgi_puzzle_game_select (Utilities|Casting|CastToGI_PuzzleGameSelect (Game|GetGameInstance)))
  (Utilities|IsValid (Variables|/Game/GameBPs/GI_PuzzleGameSelect.GI_PuzzleGameSelect_C|GetSaveRef _asgi_puzzle_game_select)
    (:Is%20Valid
      (Variables|Default|SetSaveGameRef (Variables|/Game/GameBPs/GI_PuzzleGameSelect.GI_PuzzleGameSelect_C|GetSaveRef _asgi_puzzle_game_select))
      (Variables|Default|SetSingle%20Color (Variables|/Game/PlayerBPs/SaveGame/SG_PlayerProgress.SG_PlayerProgress_C|GetbSingleColor (Variables|/Game/GameBPs/GI_PuzzleGameSelect.GI_PuzzleGameSelect_C|GetSaveRef _asgi_puzzle_game_select)))
      (if (Variables|/Game/PlayerBPs/SaveGame/SG_PlayerProgress.SG_PlayerProgress_C|GetbSingleColor (Variables|/Game/GameBPs/GI_PuzzleGameSelect.GI_PuzzleGameSelect_C|GetSaveRef _asgi_puzzle_game_select))
        (bind _output_get (Variables|Default|SetBlockColorVariable (Variables|/Game/PlayerBPs/SaveGame/SG_PlayerProgress.SG_PlayerProgress_C|GetBlockColorValue (Variables|/Game/GameBPs/GI_PuzzleGameSelect.GI_PuzzleGameSelect_C|GetSaveRef _asgi_puzzle_game_select))))
        (bind _returnvalue (Rendering|Material|CreateDynamicMaterialInstance "/Game/Materials/Material/Block_Colors.Block_Colors" "None" "None" :!class /Script/Engine.KismetMaterialLibrary))
        (Rendering|Material|SetVectorParameterValue _returnvalue "BlockColor" _output_get :!class /Script/Engine.MaterialInstanceDynamic)
        (Variables|Default|SetPlayersMaterialPref _returnvalue)
        (bind _returnvalue_2 (Rendering|Material|CreateDynamicMaterialInstance "/Game/Materials/Material/Block_Colors.Block_Colors" "Outline" "None" :!class /Script/Engine.KismetMaterialLibrary))
        (Rendering|Material|SetVectorParameterValue _returnvalue_2 "BlockColor" (Variables|/Game/PlayerBPs/SaveGame/SG_PlayerProgress.SG_PlayerProgress_C|GetOutlineColorValue (Variables|/Game/GameBPs/GI_PuzzleGameSelect.GI_PuzzleGameSelect_C|GetSaveRef _asgi_puzzle_game_select)) :!class /Script/Engine.MaterialInstanceDynamic)
        (Variables|Default|SetOutlineColor _returnvalue_2)
        (Variables|Default|SetSaveGameRef (Variables|/Game/GameBPs/GI_PuzzleGameSelect.GI_PuzzleGameSelect_C|GetSaveRef _asgi_puzzle_game_select))
        (else
          (Utilities|Array|Clear (Variables|Default|GetListOfMaterialFavorites))
          (for (_array_element _array_index) (Variables|/Game/PlayerBPs/SaveGame/SG_PlayerProgress.SG_PlayerProgress_C|GetPlayerMultiColors (Variables|/Game/GameBPs/GI_PuzzleGameSelect.GI_PuzzleGameSelect_C|GetSaveRef _asgi_puzzle_game_select))
            (Utilities|Array|SetArrayElem (Variables|Default|GetListOfColorFavorites) _array_index _array_element)
            (bind _returnvalue_3 (Rendering|Material|CreateDynamicMaterialInstance "/Game/Materials/Material/Block_Colors.Block_Colors" "None" "None" :!class /Script/Engine.KismetMaterialLibrary))
            (Rendering|Material|SetVectorParameterValue _returnvalue_3 "BlockColor" _array_element :!class /Script/Engine.MaterialInstanceDynamic)
            (Utilities|Array|Add (Variables|Default|GetListOfMaterialFavorites) _returnvalue_3))
          (bind _returnvalue_4 (Rendering|Material|CreateDynamicMaterialInstance "/Game/Materials/Material/Block_Colors.Block_Colors" "Outline" "None" :!class /Script/Engine.KismetMaterialLibrary))
          (Rendering|Material|SetVectorParameterValue _returnvalue_4 "BlockColor" (Variables|/Game/PlayerBPs/SaveGame/SG_PlayerProgress.SG_PlayerProgress_C|GetOutlineColorValue (Variables|/Game/GameBPs/GI_PuzzleGameSelect.GI_PuzzleGameSelect_C|GetSaveRef _asgi_puzzle_game_select)) :!class /Script/Engine.MaterialInstanceDynamic)
          (Variables|Default|SetOutlineColor _returnvalue_4)
          (Variables|Default|SetSaveGameRef (Variables|/Game/GameBPs/GI_PuzzleGameSelect.GI_PuzzleGameSelect_C|GetSaveRef _asgi_puzzle_game_select))
          (bind _returnvalue_5 (Actor|GetActorOfClass "/Game/GameBPs/BP_ThumbnailStudio.BP_ThumbnailStudio_C"))
          (Default|CreateThumbnails _returnvalue_5))))))

(event Custom|SmoothCameraRot
  (Utilities|FlowControl|Sequence
    (:then_0
      (Variables|Default|SetStartRotation (Pawn|GetControlRotation :!class /Script/Engine.Controller))
      (bind _newtrack_0 (Timeline|TL_EndCameraPan PlayFromStart)
        (:Update
          (Pawn|SetControlRotation (Math|Rotator|Lerp(Rotator) (Variables|Default|GetStartRotation) (Variables|Default|GetEndGameRot) _newtrack_0 true)))
        (:Finished
          (CallFunction|EndGamePieceHighlight))))))

(event Custom|EndGamePieceHighlight
  (params (GetItem :type Integer))
  (bind _returnvalue (- GetItem 1))
  (bind _endgameref (Variables|Default|GetEndGameRef))
  (bind _hudref (Variables|Default|GetHUDRef))
  (bind _wbp_inventorypanel (Variables|/Game/PlayerBPs/PlayerHUD/WBP_PlayGameHUD.WBP_PlayGameHUD_C|GetWBP_InventoryPanel _hudref))
  (bind _gamepiecesarray (Variables|/Game/PlayerBPs/PlayerHUD/WBP_InventoryPanel.WBP_InventoryPanel_C|GetGamePiecesArray _wbp_inventorypanel))
  (bind _output (Utilities|Array|Get(acopy) _gamepiecesarray _returnvalue))
  (bind _output_2 (Utilities|Array|Get(acopy) _gamepiecesarray GetItem))
  (bind _hism_cubes (Variables|/Game/GameBPs/BP_Piece.BP_Piece_C|GetHISM_Cubes _output_2))
  (bind _hism_cubes_2 (Variables|/Game/GameBPs/BP_Piece.BP_Piece_C|GetHISM_Cubes _output))
  (Utilities|FlowControl|Sequence
    (:then_0
      (if (!= GetItem 0)
        (Rendering|Material|SetMaterial _hism_cubes_2 0 (Variables|/Game/GameBPs/BP_Piece.BP_Piece_C|GetDynamicMaterial _output))
        (Rendering|Material|SetMaterial _hism_cubes_2 1 "/Game/Materials/Material_Instances/Black_Outline.Black_Outline")))
    (:then_1
      (if (< GetItem (Utilities|Array|Length _gamepiecesarray))
        (Rendering|Material|SetMaterial _hism_cubes 0 "/Game/Materials/Material/SThr_WhiteMat.SThr_WhiteMat")
        (Rendering|Material|SetMaterial _hism_cubes 1 "/Game/Materials/Material/SThr_BlackMat1.SThr_BlackMat1")
        (Utilities|FlowControl|Delay 0.4)
        (CallFunction|EndGamePieceHighlight (+ GetItem 1))
        (else
          (Utilities|FlowControl|Delay 0.75)
          (Widget|SetVisibility _endgameref "Visible")
          (Default|AnimateStars _endgameref 1))))))

(event Custom|PlayTutorial
  (bind _returnvalue (UserInterface|CreateWidget "/Game/PlayerBPs/PlayerHUD/WBP_InteractiveTutorial.WBP_InteractiveTutorial_C"))
  (Variables|Default|SetTutorialWidget _returnvalue)
  (UserInterface|Viewport|AddtoViewport _returnvalue 0))

(event Custom|CanSwitch
  (if (> (Utilities|Time|GetGameTimeinSeconds) 4.0)
    (if (not (Variables|Default|GetTutorialActive))
      (Widget|SetVisibility (Variables|Default|GetHUDControllerRef) "Visible")
      (Widget|RemovefromParent (Variables|Default|GetWBP_BeginRef)))
    (else
      (Utilities|FlowControl|Delay 0.25)
      (CallFunction|CanSwitch))))

(event Custom|TutorialInventorySelect)

(event Custom|TutorialShowHUD
  (Widget|SetVisibility (Variables|Default|GetHUDControllerRef) "Visible"))

(event EventBeginPlay
  (bind _returnvalue (Actor|GetActorOfClass "/Game/GameBPs/BP_BoardManager.BP_BoardManager_C"))
  (Utilities|IsValid _returnvalue
    (:Is%20Valid
      (bind _asgi_puzzle_game_select (Utilities|Casting|CastToGI_PuzzleGameSelect (Game|GetGameInstance)))
      (if (Variables|/Game/PlayerBPs/SaveGame/SG_PlayerProgress.SG_PlayerProgress_C|GetTutorialComplete (Variables|/Game/GameBPs/GI_PuzzleGameSelect.GI_PuzzleGameSelect_C|GetSaveRef _asgi_puzzle_game_select))
        (bind _returnvalue_2 (UserInterface|CreateWidget "/Game/PlayerBPs/PlayerHUD/WBP_BeginGame.WBP_BeginGame_C"))
        (Variables|Default|SetWBP_BeginRef _returnvalue_2)
        (UserInterface|Viewport|AddtoViewport _returnvalue_2 0)
        (else
          (CallFunction|PlayTutorial)
          (Variables|Default|SetTutorialActive true))))
    (:Is%20Not%20Valid
      _))
  (Utilities|Map|Clear (Variables|Default|GetIDtoMaterialMap))
  (bind _asgi_puzzle_game_select_2 (Utilities|Casting|CastToGI_PuzzleGameSelect (Game|GetGameInstance)))
  (Utilities|IsValid (Variables|/Game/GameBPs/GI_PuzzleGameSelect.GI_PuzzleGameSelect_C|GetSaveRef _asgi_puzzle_game_select_2)
    (:Is%20Valid
      (Variables|Default|SetSaveGameRef (Variables|/Game/GameBPs/GI_PuzzleGameSelect.GI_PuzzleGameSelect_C|GetSaveRef _asgi_puzzle_game_select_2))
      (Variables|Default|SetSingle%20Color (Variables|/Game/PlayerBPs/SaveGame/SG_PlayerProgress.SG_PlayerProgress_C|GetbSingleColor (Variables|/Game/GameBPs/GI_PuzzleGameSelect.GI_PuzzleGameSelect_C|GetSaveRef _asgi_puzzle_game_select_2)))
      (if (Variables|/Game/PlayerBPs/SaveGame/SG_PlayerProgress.SG_PlayerProgress_C|GetbSingleColor (Variables|/Game/GameBPs/GI_PuzzleGameSelect.GI_PuzzleGameSelect_C|GetSaveRef _asgi_puzzle_game_select_2))
        (bind _output_get (Variables|Default|SetBlockColorVariable (Variables|/Game/PlayerBPs/SaveGame/SG_PlayerProgress.SG_PlayerProgress_C|GetBlockColorValue (Variables|/Game/GameBPs/GI_PuzzleGameSelect.GI_PuzzleGameSelect_C|GetSaveRef _asgi_puzzle_game_select_2))))
        (bind _returnvalue_3 (Rendering|Material|CreateDynamicMaterialInstance "/Game/Materials/Material/Block_Colors.Block_Colors" "None" "None" :!class /Script/Engine.KismetMaterialLibrary))
        (Rendering|Material|SetVectorParameterValue _returnvalue_3 "BlockColor" _output_get :!class /Script/Engine.MaterialInstanceDynamic)
        (Variables|Default|SetPlayersMaterialPref _returnvalue_3)
        (bind _returnvalue_4 (Rendering|Material|CreateDynamicMaterialInstance "/Game/Materials/Material/Block_Colors.Block_Colors" "Outline" "None" :!class /Script/Engine.KismetMaterialLibrary))
        (Rendering|Material|SetVectorParameterValue _returnvalue_4 "BlockColor" (Variables|/Game/PlayerBPs/SaveGame/SG_PlayerProgress.SG_PlayerProgress_C|GetOutlineColorValue (Variables|/Game/GameBPs/GI_PuzzleGameSelect.GI_PuzzleGameSelect_C|GetSaveRef _asgi_puzzle_game_select_2)) :!class /Script/Engine.MaterialInstanceDynamic)
        (Variables|Default|SetOutlineColor _returnvalue_4)
        (Variables|Default|SetSaveGameRef (Variables|/Game/GameBPs/GI_PuzzleGameSelect.GI_PuzzleGameSelect_C|GetSaveRef _asgi_puzzle_game_select_2))
        (else
          (Utilities|Array|Clear (Variables|Default|GetListOfMaterialFavorites))
          (for (_array_element _array_index) (Variables|/Game/PlayerBPs/SaveGame/SG_PlayerProgress.SG_PlayerProgress_C|GetPlayerMultiColors (Variables|/Game/GameBPs/GI_PuzzleGameSelect.GI_PuzzleGameSelect_C|GetSaveRef _asgi_puzzle_game_select_2))
            (Utilities|Array|SetArrayElem (Variables|Default|GetListOfColorFavorites) _array_index _array_element)
            (bind _returnvalue_5 (Rendering|Material|CreateDynamicMaterialInstance "/Game/Materials/Material/Block_Colors.Block_Colors" "None" "None" :!class /Script/Engine.KismetMaterialLibrary))
            (Rendering|Material|SetVectorParameterValue _returnvalue_5 "BlockColor" _array_element :!class /Script/Engine.MaterialInstanceDynamic)
            (Utilities|Array|Add (Variables|Default|GetListOfMaterialFavorites) _returnvalue_5))
          (bind _returnvalue_6 (Rendering|Material|CreateDynamicMaterialInstance "/Game/Materials/Material/Block_Colors.Block_Colors" "Outline" "None" :!class /Script/Engine.KismetMaterialLibrary))
          (Rendering|Material|SetVectorParameterValue _returnvalue_6 "BlockColor" (Variables|/Game/PlayerBPs/SaveGame/SG_PlayerProgress.SG_PlayerProgress_C|GetOutlineColorValue (Variables|/Game/GameBPs/GI_PuzzleGameSelect.GI_PuzzleGameSelect_C|GetSaveRef _asgi_puzzle_game_select_2)) :!class /Script/Engine.MaterialInstanceDynamic)
          (Variables|Default|SetOutlineColor _returnvalue_6)
          (Variables|Default|SetSaveGameRef (Variables|/Game/GameBPs/GI_PuzzleGameSelect.GI_PuzzleGameSelect_C|GetSaveRef _asgi_puzzle_game_select_2))
          (bind _returnvalue_7 (Actor|GetActorOfClass "/Game/GameBPs/BP_ThumbnailStudio.BP_ThumbnailStudio_C"))
          (Default|CreateThumbnails _returnvalue_7))))))

(fn ConstructionScript)