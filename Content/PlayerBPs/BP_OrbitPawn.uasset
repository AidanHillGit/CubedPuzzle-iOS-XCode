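; Touch-driven player pawn for the 3D puzzle game, orbiting a camera around the board, framed by puzzle size.
; Finger traces prioritize move-gizmo arrows, then pieces, which need a short timed hold to select, then orbit.
; Orbit applies saved sensitivity with pitch limits, two-finger pinch adjusts FOV, and some actions advance the tutorial.
; Joystick moves match swipes to screen-projected world X/Y axes by dot product, then drive the active piece.
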(event Custom|Position_Update
  (params (UpdatePosition :type Vector%202D%20Structure))
  (bind _playerssensitivity (Variables|Default|GetPlayersSensitivity))
  (bind _initiallocation (Variables|Default|GetInitialLocation))
  (bind _returnvalue (- UpdatePosition _initiallocation))
  (bind _returnvalue_2 (/ _returnvalue _playerssensitivity))
  ;[0.15 0.15 0.15 0.5] Player Movement, Orbit, select, and arrow selection + pinch when a second finger is on the screen
  ;;[0 0.09759 0.5841 0.5] Update Position and Sensitivety Setting
  (if (or (Utilities|Enum|Equal(Enum) (Variables|Default|GetTouchAction) "NewEnumerator4") (Utilities|Enum|Equal(Enum) (Variables|Default|GetTouchAction) "NewEnumerator0"))
    ;;;[0.15 0.15 0.15 0.5] Orbit Controls Set up with player sensitivity
    (Utilities|FlowControl|Sequence
      (:then_0
        (Variables|Default|SetTouchAction "NewEnumerator4")
        ;;;;[0.3512 0.4573 1 0.5] Make Sure the player does not look directly below or above the piece, was causing people to get "lost"
        (Pawn|Input|AddControllerYawInput (.x _returnvalue_2))
        (if (>= (.y _returnvalue_2) 0.0)
          (if (> (Math|Rotator|NormalizeAxis (.Pitch (Math|Rotator|BreakRotator (Pawn|GetControlRotation :!class /Script/Engine.Pawn)))) -6e+01)
            (Pawn|Input|AddControllerPitchInput (.y _returnvalue_2)))
          (elif (not (> (Math|Rotator|NormalizeAxis (.Pitch (Math|Rotator|BreakRotator (Pawn|GetControlRotation :!class /Script/Engine.Pawn)))) 6e+01))
            (Pawn|Input|AddControllerPitchInput (.y _returnvalue_2)))))
      (:then_1
        ;;;[0.02956 0.107 0.1095] Play Next Section if tutorial is active
        (if (Variables|Default|GetTutorial%20Active)
          (bind _asbp_player_controller (Utilities|Casting|CastToBP_PlayerController (Game|GetPlayerController 0)))
          (if (== (Variables|/Game/PlayerBPs/PlayerHUD/WBP_InteractiveTutorial.WBP_InteractiveTutorial_C|GetTutorialStep (Variables|/Game/PlayerBPs/BP_PlayerController.BP_PlayerController_C|GetTutorialWidget _asbp_player_controller)) 0)
            (Default|Tutorial2Now (Variables|/Game/PlayerBPs/BP_PlayerController.BP_PlayerController_C|GetTutorialWidget _asbp_player_controller))))))))

(event Custom|Increase%20Score
  (params (Inc%20Score%20Value :type Integer))
  ;[0.03955 0.6514 0 0.5] GAME SETUP: Players Settings and Player Location Based Off Board Size
  ;;[1 1 1 0.5] Fill Game Score Tracker
  (Variables|Default|SetFillTheBoardScore (+ Inc%20Score%20Value (Variables|Default|GetFillTheBoardScore))))

(event Custom|MovePieceArrows
  (bind _returnvalue (Game|GetPlayerController 0))
  ;[0.15 0.15 0.15 0.5] Player Movement, Orbit, select, and arrow selection + pinch when a second finger is on the screen
  ;;[0.15 0.15 0.15 0.5] Check What The Player Tapped, Interaction with Arrows, then piece if none then allow orbit
  (if (.bBlockingHit (Collision|BreakHitResult (.HitResult (Class|PlayerController|GetHitResultUnderFingerbyChannel _returnvalue (stale Input|TouchEvents|InputTouch FingerIndex) "TraceTypeQuery3" true))))
    (Variables|Default|SetTouchAction "NewEnumerator1")
    (bind _asbp_move_gizmo (Utilities|Casting|CastToBP_MoveGizmo (.HitActor (Collision|BreakHitResult (.HitResult (Class|PlayerController|GetHitResultUnderFingerbyChannel _returnvalue (stale Input|TouchEvents|InputTouch FingerIndex) "TraceTypeQuery3" true))))))
    (Default|HitCapsule _asbp_move_gizmo (.HitComponent (Collision|BreakHitResult (.HitResult (Class|PlayerController|GetHitResultUnderFingerbyChannel _returnvalue (stale Input|TouchEvents|InputTouch FingerIndex) "TraceTypeQuery3" true)))))
    (if (Math|Boolean|ORBoolean (== (.HitComponent (Collision|BreakHitResult (.HitResult (Class|PlayerController|GetHitResultUnderFingerbyChannel _returnvalue (stale Input|TouchEvents|InputTouch FingerIndex) "TraceTypeQuery3" true)))) (Variables|/Game/GameBPs/BP_MoveGizmo.BP_MoveGizmo_C|GetCap_XNeg _asbp_move_gizmo)) (== (.HitComponent (Collision|BreakHitResult (.HitResult (Class|PlayerController|GetHitResultUnderFingerbyChannel _returnvalue (stale Input|TouchEvents|InputTouch FingerIndex) "TraceTypeQuery3" true)))) (Variables|/Game/GameBPs/BP_MoveGizmo.BP_MoveGizmo_C|GetCap_XPos _asbp_move_gizmo)) (== (.HitComponent (Collision|BreakHitResult (.HitResult (Class|PlayerController|GetHitResultUnderFingerbyChannel _returnvalue (stale Input|TouchEvents|InputTouch FingerIndex) "TraceTypeQuery3" true)))) (Variables|/Game/GameBPs/BP_MoveGizmo.BP_MoveGizmo_C|GetCap_YNeg _asbp_move_gizmo)) (== (.HitComponent (Collision|BreakHitResult (.HitResult (Class|PlayerController|GetHitResultUnderFingerbyChannel _returnvalue (stale Input|TouchEvents|InputTouch FingerIndex) "TraceTypeQuery3" true)))) (Variables|/Game/GameBPs/BP_MoveGizmo.BP_MoveGizmo_C|GetCap_YPos _asbp_move_gizmo)) (== (.HitComponent (Collision|BreakHitResult (.HitResult (Class|PlayerController|GetHitResultUnderFingerbyChannel _returnvalue (stale Input|TouchEvents|InputTouch FingerIndex) "TraceTypeQuery3" true)))) (Variables|/Game/GameBPs/BP_MoveGizmo.BP_MoveGizmo_C|GetCap_ZNeg _asbp_move_gizmo)) (== (.HitComponent (Collision|BreakHitResult (.HitResult (Class|PlayerController|GetHitResultUnderFingerbyChannel _returnvalue (stale Input|TouchEvents|InputTouch FingerIndex) "TraceTypeQuery3" true)))) (Variables|/Game/GameBPs/BP_MoveGizmo.BP_MoveGizmo_C|GetCap_ZPos _asbp_move_gizmo)))
      (Variables|Default|SetbCapsuleHit true)
      (if (Variables|Default|GetTutorial%20Active)
        (CallFunction|PlayNextTutorial)))
    (elif (.bBlockingHit (Collision|BreakHitResult (.HitResult (Class|PlayerController|GetHitResultUnderFingerbyChannel _returnvalue (stale Input|TouchEvents|InputTouch FingerIndex) "TraceTypeQuery4" true))))
      (Variables|Default|SetTouchAction "NewEnumerator2")
      (CallFunction|StartTimer)
      (Variables|Default|SetfHoldTime 0.0)
      (else
        (Variables|Default|SetTouchAction "NewEnumerator0")))))

(event Custom|StartTutorial2
  ;[0.02956 0.107 0.1095] Tutorial Based Code
  ;;[1 1 1 0.5] Start Next Tutorial Section
  (if (not (Variables|/Game/PlayerBPs/SaveGame/SG_PlayerProgress.SG_PlayerProgress_C|GetTutorialComplete (Variables|Default|GetSave%20Ref)))
    (bind _asgi_puzzle_game_select (Utilities|Casting|CastToGI_PuzzleGameSelect (Game|GetGameInstance)))
    (if (== (Variables|/Game/GameBPs/GI_PuzzleGameSelect.GI_PuzzleGameSelect_C|GetTutorialStep _asgi_puzzle_game_select) 0)
      (Variables|/Game/GameBPs/GI_PuzzleGameSelect.GI_PuzzleGameSelect_C|SetTutorialStep _asgi_puzzle_game_select 1))))

(event Custom|StartTimer
  ;[0.65 0.325 0.65 0.5] Hold Piece To Switch To A Piece on board. Players would switch to a piece by accident when clicking a piece. Holding prevents that issue
  (bind _output_get (Variables|Default|SetbActiveHold true))
  (bind _returnvalue (Utilities|Time|SetTimerbyEvent (delegate Custom|HoldingPiece) 0.05 _output_get))
  (Variables|Default|SetHoldingEventHandle _returnvalue))

(event Custom|HoldingPiece
  ;[0.65 0.325 0.65 0.5] Hold Piece To Switch To A Piece on board. Players would switch to a piece by accident when clicking a piece. Holding prevents that issue
  (if (and (.ReturnValue (Class|PlayerController|GetHitResultUnderFingerbyChannel (Game|GetPlayerController 0) (stale Input|TouchEvents|InputTouch FingerIndex) "TraceTypeQuery4" true)) (Variables|Default|GetbActiveHold))
    (if (>= (Variables|Default|GetfHoldTime) 0.19)
      (bind _asbp_piece (Utilities|Casting|CastToBP_Piece (.HitActor (Collision|BreakHitResult (.HitResult (Class|PlayerController|GetHitResultUnderFingerbyChannel (Game|GetPlayerController 0) (stale Input|TouchEvents|InputTouch FingerIndex) "TraceTypeQuery4" true))))))
      (Utilities|IsValid (Variables|/Game/GameBPs/BP_Piece.BP_Piece_C|GetWidgetRef _asbp_piece)
        (:Is%20Valid
          (Default|SelectedinGame (Variables|/Game/GameBPs/BP_Piece.BP_Piece_C|GetWidgetRef _asbp_piece))
          (Utilities|Time|ClearandInvalidateTimerbyHandle (Variables|Default|GetHoldingEventHandle)) ; End Event Timer Stopping From Selecting a piece behind this one
        ))
      (else
        (Variables|Default|SetfHoldTime (+ (Variables|Default|GetfHoldTime) 0.05))))))

(event Custom|PlayNextTutorial
  ;[0.02956 0.107 0.1095] Tutorial Based Code
  ;;[1 1 1 0.5] Play Tutorial if it is active and not completed
  (if (not (Variables|/Game/PlayerBPs/SaveGame/SG_PlayerProgress.SG_PlayerProgress_C|GetTutorialComplete (Variables|Default|GetSave%20Ref)))
    (bind _asbp_player_controller (Utilities|Casting|CastToBP_PlayerController (Game|GetPlayerController 0)))
    (if (== (Variables|/Game/PlayerBPs/PlayerHUD/WBP_InteractiveTutorial.WBP_InteractiveTutorial_C|GetTutorialStep (Variables|/Game/PlayerBPs/BP_PlayerController.BP_PlayerController_C|GetTutorialWidget _asbp_player_controller)) 2)
      (Default|TutorialEvent4 (Variables|/Game/PlayerBPs/BP_PlayerController.BP_PlayerController_C|GetTutorialWidget _asbp_player_controller)))))

(event Custom|Move%20Piece%20AutoDirection
  (params (SwipeDelta :type Vector%202D%20Structure))
  (bind _bp_moveref (Variables|Default|GetBP_MoveRef))
  ;[0.15 0.15 0.15 0.5] Move Piece From Joystick Controls
  (Utilities|IsValid (Variables|/Game/GameBPs/BP_MoveGizmo.BP_MoveGizmo_C|GetPieceRef _bp_moveref)
    (:Is%20Valid
      _)
    (:Is%20Not%20Valid
      (Utilities|IsValid (Variables|/Game/GameBPs/BP_MoveGizmo.BP_MoveGizmo_C|GetFillPieceRef _bp_moveref)
        (:Is%20Valid
          _))))
  (Variables|Default|SetbMovedPiece true)
  (bind (_screenposx1 _screennegx1 _screenposy1 _screennegy1) (CallFunction|UpdateDragDirection))
  (bind _returnvalue (CallFunction|GetSwipeDirection SwipeDelta _screenposx1 _screennegx1 _screenposy1 _screennegy1))
  (bind _output_get (Variables|Default|SetLastMoveIndex _returnvalue))
  (if (not (== _output_get -1))
    (Default|MoveorRotatePiece (Variables|Default|GetBP_MoveRef) (Variables|Default|GetLastMoveIndex))
    (Variables|Default|SetLastMoveIndex -1)))

(event EventBeginPlay
  (bind _puzzlecenterref (Variables|Default|GetPuzzleCenterRef))
  ;[0.03955 0.6514 0 0.5] GAME SETUP: Players Settings and Player Location Based Off Board Size
  (Utilities|FlowControl|Sequence
    (:then_0
      (Utilities|IsValid (Variables|Default|GetPuzzleCenterRef)
        (:Is%20Valid
          (if (not (== (Utilities|GetClass (Game|GetGameMode)) "/Game/PlayerBPs/MenuGameMode.MenuGameMode_C"))
            (Variables|/Script/Engine.SpringArmComponent|SetTargetArmLength (Variables|Default|GetSpringArm) (+ (Math|Conversions|ToFloat(Integer) (* 55 (Variables|/Game/GameBPs/BP_BoardManager.BP_BoardManager_C|GetPuzzleSizeN (Variables|Default|GetPuzzleCenterRef)))) 4e+02))
            (Variables|Default|SetPlayerZoom 1.2e+02)
            (if (== (Math|Integer|%(Integer) (Variables|/Game/GameBPs/BP_BoardManager.BP_BoardManager_C|GetPuzzleSizeN _puzzlecenterref) 2) 0)
              (Transformation|SetActorLocation (Math|Conversions|ToVector(Float) (/ (Variables|/Game/GameBPs/BP_BoardManager.BP_BoardManager_C|GetCellSize _puzzlecenterref) 2.0)) false false)
              (else
                (Transformation|SetActorLocation "0, 0, 0" false false)))))
        (:Is%20Not%20Valid
          (Utilities|IsValid "/Game/GameBPs/FillTheCubeBPS/BP_FillTheCubeBoard.BP_FillTheCubeBoard"
            (:Is%20Valid
              (bind _returnvalue (Actor|GetActorOfClass "/Game/GameBPs/FillTheCubeBPS/BP_FillTheCubeBoard.BP_FillTheCubeBoard_C"))
              (Variables|Default|SetFillBoard_Ref _returnvalue)
              (if (not (== (Utilities|GetClass (Game|GetGameMode)) "/Game/PlayerBPs/MenuGameMode.MenuGameMode_C"))
                (Variables|/Script/Engine.SpringArmComponent|SetTargetArmLength (Variables|Default|GetSpringArm) (+ (Math|Conversions|ToFloat(Integer) (* 55 (Variables|/Game/GameBPs/FillTheCubeBPS/BP_FillTheCubeBoard.BP_FillTheCubeBoard_C|GetPuzzleSizeN (Variables|Default|GetFillBoard_Ref)))) 7.5e+02))
                (Variables|Default|SetPlayerZoom 1.2e+02)
                (if (== (Math|Integer|%(Integer) (Variables|/Game/GameBPs/FillTheCubeBPS/BP_FillTheCubeBoard.BP_FillTheCubeBoard_C|GetPuzzleSizeN (Variables|Default|GetFillBoard_Ref)) 2) 0)
                  (Transformation|SetActorLocation (Math|Conversions|ToVector(Float) (/ (Variables|/Game/GameBPs/FillTheCubeBPS/BP_FillTheCubeBoard.BP_FillTheCubeBoard_C|GetCellSize (Variables|Default|GetFillBoard_Ref)) 2.0)) false false)
                  (else
                    (Transformation|SetActorLocation "0, 0, 0" false false)))))))))
    (:then_1
      ;;[1 1 1 0.5] Get Game save and set tutorial save ref
      (bind _asgi_puzzle_game_select (Utilities|Casting|CastToGI_PuzzleGameSelect (Game|GetGameInstance)))
      (Default|LoadorCreateSave _asgi_puzzle_game_select "PlayersLevelProgress")
      (Variables|Default|SetPlayersSensitivity (Variables|/Game/PlayerBPs/SaveGame/SG_PlayerProgress.SG_PlayerProgress_C|GetPlayersSens (Variables|/Game/GameBPs/GI_PuzzleGameSelect.GI_PuzzleGameSelect_C|GetSaveRef _asgi_puzzle_game_select)))
      (Variables|Default|SetSave%20Ref (Variables|/Game/GameBPs/GI_PuzzleGameSelect.GI_PuzzleGameSelect_C|GetSaveRef _asgi_puzzle_game_select))
      (Variables|Default|SetTutorial%20Active (Variables|/Game/GameBPs/GI_PuzzleGameSelect.GI_PuzzleGameSelect_C|GetbTutorialActive _asgi_puzzle_game_select)))))

(event Input|TouchEvents|Touch2
  (params (Key :type Key%20Structure :default "None"))
  ;[0.15 0.15 0.15 0.5] Player Movement, Orbit, select, and arrow selection + pinch when a second finger is on the screen
  ;;[0.15 0.15 0.15 0.5] Zoom in and Out
  (:Pressed
    (Variables|Default|SetintStartDistance (.Distance (CallFunction|ZoomTouch)))))

(event Input|KeyboardEvents|GesturePinch
  (params (Key :type Key%20Structure :default "None"))
  ;[0.15 0.15 0.15 0.5] Player Movement, Orbit, select, and arrow selection + pinch when a second finger is on the screen
  ;;[0.15 0.15 0.15 0.5] Check What The Player Tapped, Interaction with Arrows, then piece if none then allow orbit
  ;;;[0.15 0.15 0.15 0.5] Zoom in and Out
  (:Pressed
    (Variables|Default|SetPinchMode true)
    (Variables|Default|SetCanMove false))
  (:Released
    (Variables|Default|SetPinchMode false)
    (Utilities|FlowControl|Delay 0.1)
    (Variables|Default|SetCanMove true)))

(event Input|TouchEvents|InputTouch
  (params (Location :type Vector) (FingerIndex :type ETouchIndex%20Enum))
  (bind (_x _y) (Math|Vector|BreakVector Location))
  (bind (_x_2 _y_2) (Math|Vector|BreakVector Location))
  (bind _doubletouch (CallFunction|ZoomTouch))
  (bind (_doubletouch_2 _distance) (CallFunction|ZoomTouch))
  (bind _bgameover_ (Variables|Default|GetbGameOver?))
  (bind _playercamera (Variables|Default|GetPlayerCamera))
  (bind _pinchmode (Variables|Default|GetPinchMode))
  (bind _bp_moveref (Variables|Default|GetBP_MoveRef))
  (bind _returnvalue (Math|Boolean|ORBoolean _bgameover_ _doubletouch _pinchmode))
  (bind _fieldofview (Variables|/Script/Engine.CameraComponent|GetFieldOfView _playercamera))
  ;[0.15 0.15 0.15 0.5] Player Movement, Orbit, select, and arrow selection + pinch when a second finger is on the screen
  (:Pressed
    (if (not _returnvalue)
      (Variables|Default|SetInitialLocation (Math|Vector2D|MakeVector2D _x _y))
      (CallFunction|MovePieceArrows)))
  (:Released
    (Variables|Default|SetLastMoveIndex -1)
    (Variables|Default|SetbActiveHold false)
    (Variables|Default|SetbMovedPiece false)
    (Variables|Default|SetfHoldTime 0.0)
    (if (not _returnvalue)
      (Variables|Default|SetbCapsuleHit false)
      (if (Variables|Default|GetbCanSwitch)
        ;;[0.15 0.15 0.15 0.5] Switch From Move To Rotate
        (Variables|/Game/GameBPs/BP_MoveGizmo.BP_MoveGizmo_C|SetbMoveMode _bp_moveref (not (Variables|/Game/GameBPs/BP_MoveGizmo.BP_MoveGizmo_C|GetbMoveMode _bp_moveref)))
        (elif (not (Variables|Default|GetPinchMode))
          (Variables|Default|SetCurrentLocation (Variables|Default|GetInitialLocation))
          (Variables|Default|SetLastTapTime (Utilities|Time|GetRealTimeSeconds))))))
  (:Moved
    (if _returnvalue
      ;;[0.15 0.15 0.15 0.5] Zoom in and Out
      (if _doubletouch_2
        (if (< (Variables|Default|GetintStartDistance) _distance)
          (CallFunction|SetCameraFOV (Math|Float|Clamp(Float) (- _fieldofview 0.5) 8e+01 1.5e+02))
          (else
            (CallFunction|SetCameraFOV (Math|Float|Clamp(Float) (+ _fieldofview 0.5) 8e+01 1.5e+02))))
        (Utilities|FlowControl|Delay 0.5)
        (Variables|Default|SetintStartDistance (.Distance (CallFunction|ZoomTouch))))
      (else
        ;;[0.15 0.15 0.15 0.5] Orbit Player Camera
        (if (and (Variables|Default|GetbOrbitMode) (Variables|Default|GetCanMove))
          (Variables|Default|SetCurrentLocation (Math|Vector2D|MakeVector2D _x_2 _y_2))
          (CallFunction|PositionUpdate (Math|Vector2D|MakeVector2D _x_2 _y_2))
          (Variables|Default|SetInitialLocation (Math|Vector2D|MakeVector2D _x_2 _y_2)))))))

(fn ConstructionScript)

(fn SetCameraFOV
  (params (FOV :type Float%20%28double-precision%29))
  (Camera|SetFieldOfView (Variables|Default|GetPlayerCamera) FOV))

(fn UpdateGizmo
  (params (YawFloat :type Float%20%28double-precision%29))
  (bind _returnvalue (+ YawFloat 45.0))
  (bind _returnvalue_2 (Math|Float|Truncate _returnvalue))
  (bind _returnvalue_3 (/ _returnvalue_2 90))
  (if (!= (Variables|Default|GetCurrentQuadrant) _returnvalue_3)
    (bind _output_get (Variables|Default|SetCurrentQuadrant _returnvalue_3))
    (if (== (Math|Integer|%(Integer) _output_get 2) 0)
      (return true "Y")
      (else
        (return true "X")))
    (else
      (return false ""))))

(fn GetMoveDirection
  ;[0.15 0.15 0.15 0.5] Get The Swipe Direction Vertical Or Horizontal
  (bind _output_get (LocalVariables|SetDelta (- (Variables|Default|GetInitialLocation) (Variables|Default|GetEndSlide))))
  (LocalVariables|SetABS_X (Math|Float|Absolute(Float) (.X (Math|Vector2D|BreakVector2D _output_get))))
  (LocalVariables|SetABS_Y (Math|Float|Absolute(Float) (.Y (Math|Vector2D|BreakVector2D _output_get))))
  (if (> (LocalVariables|GetABS_X) (LocalVariables|GetABS_Y)) ; True = Horizontal
    (if (> (.x (Variables|Default|GetInitialLocation)) (.x (Variables|Default|GetEndSlide)))
      (return false -1)
      (else
        (return false 1)))
    (elif (> (.y (Variables|Default|GetInitialLocation)) (.y (Variables|Default|GetEndSlide)))
      (return true 1)
      (else
        (return true -1)))))

(fn UpdateMove
  (if (Variables|Default|GetbFirstMove)
    (Variables|Default|SetbFirstMove false)
    (Math|Integer|IncrementInt (Variables|/Game/GameBPs/BP_BoardManager.BP_BoardManager_C|GetMoves (Variables|Default|GetPuzzleCenterRef)))))

(fn SwitchModes
  (params (ChangeMode :type Boolean))
  (if ChangeMode
    (Variables|Default|SetbOrbitMode (not (Variables|Default|GetbOrbitMode)))))

(fn ZoomTouch
  (bind _returnvalue (Game|GetPlayerController 0))
  (bind _returnvalue_2 (Game|GetPlayerController 0))
  (bind (_locationx _locationy _biscurrentlypressed) (Class|PlayerController|GetInputTouchState _returnvalue "Touch2"))
  (bind (_locationx_2 _locationy_2 _biscurrentlypressed_2) (Class|PlayerController|GetInputTouchState _returnvalue_2 "Touch1"))
  (return (and _biscurrentlypressed_2 _biscurrentlypressed) (Math|Float|Truncate (/ (Math|Vector|Distance2D(Vector) (Math|Vector2D|MakeVector2D _locationx_2 _locationy_2) (Math|Vector2D|MakeVector2D _locationx _locationy)) 1e+02))))

(fn UpdateDragDirection
  (bind _returnvalue (Transformation|GetActorLocation))
  (bind _returnvalue_2 (Game|GetPlayerController 0))
  (bind _returnvalue_3 (Transformation|GetActorLocation))
  (bind _returnvalue_4 (Game|GetPlayerController 0))
  (bind _returnvalue_5 (+ (.y _returnvalue_3) 55.0))
  (bind _returnvalue_6 (+ (.x _returnvalue) 55.0))
  (bind _returnvalue_7 (Math|Vector|MakeVector (.x _returnvalue_3) _returnvalue_5 (.z _returnvalue_3)))
  (bind _returnvalue_8 (Math|Vector|MakeVector _returnvalue_6 (.y _returnvalue) (.z _returnvalue)))
  (bind _screenposition (Class|GameplayStatics|ProjectWorldtoScreen _returnvalue_2 _returnvalue_7 false))
  (bind _screenposition_2 (Class|GameplayStatics|ProjectWorldtoScreen _returnvalue_4 _returnvalue_8 false))
  (bind (_x _y) (Math|Vector2D|BreakVector2D _screenposition))
  (bind (_x_2 _y_2) (Math|Vector2D|BreakVector2D _screenposition_2))
  (LocalVariables|SetCenterScreen (.ScreenPosition (Class|GameplayStatics|ProjectWorldtoScreen (Game|GetPlayerController 0) (Transformation|GetActorLocation) false)))
  (bind _output_get (LocalVariables|SetXPointScreen (Math|Vector2D|MakeVector2D _x_2 _y_2)))
  (bind _output_get_2 (LocalVariables|SetXDirection (- _output_get (LocalVariables|GetCenterScreen))))
  (LocalVariables|SetScreenPosX (Math|Vector2D|Normalize2D _output_get_2))
  (LocalVariables|SetScreenNegX (* (Math|Vector2D|Normalize2D _output_get_2) "(X=-1.000000,Y=-1.000000)"))
  (bind _output_get_3 (LocalVariables|SetYPointScreen (Math|Vector2D|MakeVector2D _x _y)))
  (bind _output_get_4 (LocalVariables|SetYDirection (- _output_get_3 (LocalVariables|GetCenterScreen))))
  (LocalVariables|SetScreenPosY (Math|Vector2D|Normalize2D _output_get_4))
  (LocalVariables|SetScreenNegY (* (Math|Vector2D|Normalize2D _output_get_4) "(X=-1.000000,Y=-1.000000)"))
  (return (LocalVariables|GetScreenPosX) (LocalVariables|GetScreenNegX) (LocalVariables|GetScreenPosY) (LocalVariables|GetScreenNegY)))

(fn ExceedsDistance
  (bind _initiallocation (Variables|Default|GetInitialLocation))
  (bind _currentlocation (Variables|Default|GetCurrentLocation))
  (bind _returnvalue (- (.x _currentlocation) (.x _initiallocation)))
  (bind _returnvalue_2 (- (.y _currentlocation) (.y _initiallocation)))
  (if (> (Math|Float|Sqrt (+ (* _returnvalue _returnvalue) (* _returnvalue_2 _returnvalue_2))) 15.0)
    (bind _output_get (LocalVariables|SetSwipeDelta (Math|Vector2D|MakeVector2D _returnvalue _returnvalue_2)))
    (return true _output_get)
    (else
      (return false ""))))

(fn GetSwipeDirection
  (params (SwipeDelta :type Vector%202D%20Structure) (ScreenPosX :type Vector%202D%20Structure) (ScreenNegX :type Vector%202D%20Structure) (ScreenPosY :type Vector%202D%20Structure) (ScreenNegY :type Vector%202D%20Structure))
  (bind _returnvalue (Math|Vector2D|Normalize2D SwipeDelta))
  (if (Utilities|Operators|EqualEqual :A _returnvalue)
    (return -1)
    (else
      (bind _output_get (LocalVariables|SetDotProductScores (Utilities|Array|MakeArray (Math|Vector2D|DotProduct(2D) _returnvalue ScreenPosX) (Math|Vector2D|DotProduct(2D) _returnvalue ScreenNegX) (Math|Vector2D|DotProduct(2D) _returnvalue ScreenPosY) (Math|Vector2D|DotProduct(2D) _returnvalue ScreenNegY))))
      (LocalVariables|SetHighestScore -2.0)
      (LocalVariables|SetBestIndex -1)
      (for (_array_element _array_index) _output_get
        (if (> _array_element (LocalVariables|GetHighestScore))
          (LocalVariables|SetHighestScore _array_element)
          (LocalVariables|SetBestIndex _array_index)))
      (return (LocalVariables|GetBestIndex)))))