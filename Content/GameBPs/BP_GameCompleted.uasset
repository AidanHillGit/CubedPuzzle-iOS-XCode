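; BP_GameCompleted is a game-completion visual effect actor showing three nested holographic cubes that pulse in size and opacity.
; BeginPlay creates two dynamic Hologram_Mat instances on PusleCube's material slots and shares them with PusleCube1 and PusleCube2.
; PulsedCube uses a timeline to scale the cubes toward a given size with slight offsets between them, leaving its Margin input unused.
; AdjustOpacity animates a faint opacity override, then resets it to zero.
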(event Custom|PulsedCube
  (params (CubeSize :type Integer) (Margin :type Integer))
  (bind _puslecube (Variables|Default|GetPusleCube))
  (bind _puslecube2 (Variables|Default|GetPusleCube2))
  (bind _puslecube1 (Variables|Default|GetPusleCube1))
  (bind _newtrack_1 (Timeline|IncreaseSize PlayFromStart)
    (:Update
      (Transformation|SetRelativeScale3D _puslecube (Math|Vector|Lerp(Vector) (Variables|/Script/Engine.SceneComponent|GetRelativeScale3D _puslecube) (* CubeSize "1.000000,1.000000,1.000000") _newtrack_1))
      (Transformation|SetRelativeScale3D _puslecube1 (Math|Vector|Lerp(Vector) (Variables|/Script/Engine.SceneComponent|GetRelativeScale3D _puslecube1) (* CubeSize "1.100000,1.100000,1.100000") _newtrack_1))
      (Transformation|SetRelativeScale3D _puslecube2 (Math|Vector|Lerp(Vector) (Variables|/Script/Engine.SceneComponent|GetRelativeScale3D _puslecube2) (* CubeSize "0.900000,0.900000,0.900000") _newtrack_1)))))

(event Custom|AdjustOpacity
  (bind _newtrack_0 (Timeline|OpacityTimeline PlayFromStart)
    (:Update
      (Rendering|Material|SetScalarParameterValue (Variables|Default|GetDynamicMat1) "Opacity Override" (Math|Float|Lerp 0.0 0.03 _newtrack_0) :!class /Script/Engine.MaterialInstanceDynamic)
      (Rendering|Material|SetScalarParameterValue (Variables|Default|GetDynamicMat2) "Opacity Override" (Math|Float|Lerp 0.0 0.03 _newtrack_0) :!class /Script/Engine.MaterialInstanceDynamic))
    (:Finished
      (Rendering|Material|SetScalarParameterValue (Variables|Default|GetDynamicMat1) "Opacity Override" 0.0 :!class /Script/Engine.MaterialInstanceDynamic)
      (Rendering|Material|SetScalarParameterValue (Variables|Default|GetDynamicMat2) "Opacity Override" 0.0 :!class /Script/Engine.MaterialInstanceDynamic))))

(event EventBeginPlay
  (bind _puslecube (Variables|Default|GetPusleCube))
  (bind _returnvalue (Rendering|Material|CreateDynamicMaterialInstance _puslecube 0 "/Game/Materials/Material/Hologram_Mat.Hologram_Mat" "None" :!class /Script/Engine.PrimitiveComponent))
  (bind _output_get (Variables|Default|SetDynamicMat1 _returnvalue))
  (Rendering|Material|SetMaterial (Variables|Default|GetPusleCube1) 0 _output_get)
  (bind _returnvalue_2 (Rendering|Material|CreateDynamicMaterialInstance _puslecube 1 "/Game/Materials/Material/Hologram_Mat.Hologram_Mat" "None" :!class /Script/Engine.PrimitiveComponent))
  (bind _output_get_2 (Variables|Default|SetDynamicMat2 _returnvalue_2))
  (Rendering|Material|SetMaterial (Variables|Default|GetPusleCube1) 1 _output_get_2))

(fn ConstructionScript)