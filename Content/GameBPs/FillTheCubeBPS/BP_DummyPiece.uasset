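; BP_DummyPiece is a cube piece for the Fill The Cube puzzle that colors its mesh by PieceID.
; On BeginPlay and on request, it takes its material from the player controller's ID-to-material map, or the player's preferred material when the saved SingleColor option is on.
; It can preview a given material.
; On removal it spawns BP_GameCompleted at its transform, calls DeletePlanePiece on it, then destroys itself.
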(event Custom|RemovePieceFromGame
  (Utilities|FlowControl|Sequence
    (:then_0
      (bind _returnvalue (Game|SpawnActorfromClass "/Game/GameBPs/BP_GameCompleted.BP_GameCompleted_C" (Transformation|GetActorTransform) "Undefined" "MultiplyWithRoot" 0 0))
      (Default|DeletePlanePiece _returnvalue))
    (:then_1
      (Actor|DestroyActor))))

(event Custom|ChangeMaterialWithID
  (bind _asgi_puzzle_game_select (Utilities|Casting|CastToGI_PuzzleGameSelect (Game|GetGameInstance)))
  (if (Variables|/Game/PlayerBPs/SaveGame/SG_PlayerProgress.SG_PlayerProgress_C|GetbSingleColor (Variables|/Game/GameBPs/GI_PuzzleGameSelect.GI_PuzzleGameSelect_C|GetSaveRef _asgi_puzzle_game_select))
    (bind _asbp_player_controller (Utilities|Casting|CastToBP_PlayerController (Game|GetPlayerController 0)))
    (Rendering|Material|SetMaterial (Variables|Default|GetCubeMesh) 0 (Variables|/Game/PlayerBPs/BP_PlayerController.BP_PlayerController_C|GetPlayersMaterialPref _asbp_player_controller))
    (else
      (bind _asbp_player_controller_2 (Utilities|Casting|CastToBP_PlayerController (Game|GetPlayerController 0)))
      (Rendering|Material|SetMaterial (Variables|Default|GetCubeMesh) 0 (.Value (Utilities|Map|Find (Variables|/Game/PlayerBPs/BP_PlayerController.BP_PlayerController_C|GetIDtoMaterialMap _asbp_player_controller_2) (Variables|Default|GetPieceID)))))))

(event Custom|PreviewColor
  (params (Material :type Material%20Interface%20Object%20Reference))
  (Rendering|Material|SetMaterial (Variables|Default|GetCubeMesh) 0 Material))

(event EventBeginPlay
  (bind _asbp_player_controller (Utilities|Casting|CastToBP_PlayerController (Game|GetPlayerController 0)))
  (Rendering|Material|SetMaterial (Variables|Default|GetCubeMesh) 0 (.Value (Utilities|Map|Find (Variables|/Game/PlayerBPs/BP_PlayerController.BP_PlayerController_C|GetIDtoMaterialMap _asbp_player_controller) (Variables|Default|GetPieceID))))
  (Utilities|FlowControl|DelayUntilNextTick)
  (CallFunction|ChangeMaterialwithID))

(fn ConstructionScript)