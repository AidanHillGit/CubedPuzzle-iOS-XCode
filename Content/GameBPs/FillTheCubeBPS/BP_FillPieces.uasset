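; BP_FillPieces is a multi-cell puzzle piece for the Fill The Cube game, snapped to and registered on BP_FillTheCubeBoard.
; Pivot-relative LocalCells define its board footprint and HISM cube visual, with rotation applying integer quarter turns around the pivot.
; Drag steps it along an axis, reverting with a scale pulse if blocked, otherwise moving the gizmo and checking completion.
; PlacePiece spawns per-cell BP_DummyPiece actors inside the solve zone and returns a size-based value.
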(event Custom|PlayScalePulse
  ;[0.15 0.15 0.15 0.5] Pusling Function On Click
  (bind _newtrack_0 (Timeline|ScalePulseTimeline PlayFromStart)
    (:Update
      (Transformation|SetActorScale3D (* (Math|Vector|ClampVectorSize (Transformation|GetActorScale3D) 0.0 2.0) (Math|Vector|MakeVector _newtrack_0 _newtrack_0 _newtrack_0))))
    (:Finished
      (Transformation|SetActorScale3D "1.000000,1.000000,1.000000"))))

(event EventBeginPlay
  (bind _returnvalue (Actor|GetActorOfClass "/Game/GameBPs/FillTheCubeBPS/BP_FillTheCubeBoard.BP_FillTheCubeBoard_C"))
  (Variables|Default|SetBoardRef _returnvalue)
  (Variables|Default|SetbDragging false)
  (bind _output_get (Variables|Default|SetWorldPos (.location (Transformation|GetActorTransform))))
  (bind _cell (Default|WorldtoGridSnapped (Variables|Default|GetBoardRef) _output_get))
  (bind _output_get_2 (Variables|Default|SetAnchorCell _cell))
  (bind _world (Default|GridtoWorld (Variables|Default|GetBoardRef) _output_get_2))
  (Transformation|SetActorLocation _world false true)
  (bind _cellsout (CallFunction|ComputeBoardCellsPivot _output_get_2))
  (bind _output_get_3 (Variables|Default|SetCurrentCells _cellsout))
  (for _array_element _output_get_3
    (Default|SetCellOccupied (Variables|Default|GetBoardRef) _array_element)))

(fn ConstructionScript)

(fn InIt
  (params (BoardRefIn :type BP%20Fill%20the%20Cube%20Board%20Object%20Reference))
  (Variables|Default|SetBoardRef BoardRefIn))

(fn ComputeBoardCellsPivot
  (params (AnchorCells :type Int%20Vector%20Structure))
  (bind (_x _y _z) (Utilities|Struct|BreakIntVector AnchorCells))
  (bind _pivotlocalcell (Variables|Default|GetPivotLocalCell))
  (for _array_element (Variables|Default|GetLocalCells)
    (Utilities|Array|Add (LocalVariables|GetOutCells) (Utilities|Struct|MakeIntVector (+ _x (- (.X (Utilities|Struct|BreakIntVector _array_element)) (.x _pivotlocalcell))) (+ _y (- (.Y (Utilities|Struct|BreakIntVector _array_element)) (.y _pivotlocalcell))) (+ _z (- (.Z (Utilities|Struct|BreakIntVector _array_element)) (.z _pivotlocalcell))))))
  (return (LocalVariables|GetOutCells)))

(fn BuildVisualfromLocalCellsPivot
  (params (CellsToDraw :type Array%20of%20Int%20Vector%20Structures))
  (bind _cellsize (Variables|Default|GetCellSize))
  (bind _pivotlocalcell (Variables|Default|GetPivotLocalCell))
  (if (Utilities|Array|IsEmpty CellsToDraw)
    (Components|InstancedStaticMesh|ClearInstances (Variables|Default|GetHISM_Cubes))
    (Development|PrintString "EMPTY")
    (else
      (Components|InstancedStaticMesh|ClearInstances (Variables|Default|GetHISM_Cubes))
      (for _array_element CellsToDraw
        (Components|InstancedStaticMesh|AddInstance (Variables|Default|GetHISM_Cubes) (Math|Transform|MakeTransform (Math|Vector|MakeVector (* (- (.X (Utilities|Struct|BreakIntVector _array_element)) (.x _pivotlocalcell)) _cellsize) (* (- (.Y (Utilities|Struct|BreakIntVector _array_element)) (.y _pivotlocalcell)) _cellsize) (* (- (.Z (Utilities|Struct|BreakIntVector _array_element)) (.z _pivotlocalcell)) _cellsize)) "0, 0, 0" "0.275000,0.275000,0.275000") false)))))

(fn GetRotatedLocalCellsPivoted
  (Utilities|Array|Clear (LocalVariables|GetRotCells))
  (for _array_element (Variables|Default|GetLocalCells)
    (bind _cellout (CallFunction|RotateCellAroundPivot _array_element))
    (Utilities|Array|Add (LocalVariables|GetRotCells) _cellout))
  (return (LocalVariables|GetRotCells)))

(fn PreviewatWorld
  (params (WorldPos :type Int%20Vector%20Structure))
  (bind _boardref (Variables|Default|GetBoardRef))
  (Utilities|IsValid _boardref
    (:Is%20Valid
      (bind _cell (Default|WorldtoGridSnapped _boardref (Math|Conversions|ToVector(Float) WorldPos)))
      (bind _cellsout (CallFunction|ComputeBoardCellsPivot _cell))
      (bind _output_get (Variables|Default|SetPreviewCells _cellsout))
      (bind _bcanplace (Default|CanPlaceinSolveZone _boardref _output_get))
      (if _bcanplace
        (bind _output_get_2 (Variables|Default|SetLastValidCell _cell))
        (bind _world (Default|GridtoWorld _boardref _output_get_2))
        (bind _output_get_3 (Variables|Default|SetLastValidWorld _world))
        (Transformation|SetActorLocation _output_get_3 false true)
        (return true)
        (else
          (Variables|Default|SetAnchorCell (Variables|Default|GetLastValidCell))
          (return false))))
    (:Is%20Not%20Valid
      (return false))))

(fn Rot90X
  (params (CellIn :type Int%20Vector%20Structure))
  (bind (_x _y _z) (Utilities|Struct|BreakIntVector CellIn))
  (return (Utilities|Struct|MakeIntVector _x (* _z -1) _y)))

(fn Rot90Y
  (params (CellIn :type Int%20Vector%20Structure))
  (bind (_x _y _z) (Utilities|Struct|BreakIntVector CellIn))
  (return (Utilities|Struct|MakeIntVector _z _y (* _x -1))))

(fn Rot90Z
  (params (CellIn :type Int%20Vector%20Structure))
  (bind (_x _y _z) (Utilities|Struct|BreakIntVector CellIn))
  (return (Utilities|Struct|MakeIntVector (* _y -1) _x _z)))

(fn NormalizeCellstoZero
  (params (InCells :type Array%20of%20Int%20Vector%20Structures))
  (if (== (Utilities|Array|Length InCells) 0)
    (return 0)
    (else
      (for _array_element InCells
        (LocalVariables|SetMinX (Math|Integer|Min(Integer) (.X (Utilities|Struct|BreakIntVector _array_element)) (LocalVariables|GetMinX)))
        (LocalVariables|SetMinY (Math|Integer|Min(Integer) (.Y (Utilities|Struct|BreakIntVector _array_element)) (LocalVariables|GetMinY)))
        (LocalVariables|SetMinZ (Math|Integer|Min(Integer) (.Z (Utilities|Struct|BreakIntVector _array_element)) (LocalVariables|GetMinZ))))
      (Utilities|Array|Clear (LocalVariables|GetCellsOut))
      (for _array_element_2 InCells
        (Utilities|Array|Add (LocalVariables|GetCellsOut) (Utilities|Struct|MakeIntVector (- (.X (Utilities|Struct|BreakIntVector _array_element_2)) (LocalVariables|GetMinX)) (- (.Y (Utilities|Struct|BreakIntVector _array_element_2)) (LocalVariables|GetMinY)) (- (.Z (Utilities|Struct|BreakIntVector _array_element_2)) (LocalVariables|GetMinZ)))))
      (return (LocalVariables|GetCellsOut)))))

(fn BuildVisualfromCells
  (params (CellsToDraw :type Array%20of%20Int%20Vector%20Structures))
  (bind _hism_cubes (Variables|Default|GetHISM_Cubes))
  (bind _offset (LocalVariables|GetOffset))
  (bind (_x _y _z) (Math|Vector|BreakVector _offset))
  (Components|InstancedStaticMesh|ClearInstances _hism_cubes)
  (for _array_element CellsToDraw
    (bind _output_get (LocalVariables|SetInstanceTransform (Math|Transform|MakeTransform (Math|Vector|MakeVector (* (.x _array_element) _x) (* (.y _array_element) _y) (* (.z _array_element) _z)) "0, 0, 0" "0.275000,0.275000,0.275000")))
    (Components|InstancedStaticMesh|AddInstance _hism_cubes _output_get false))
  (Variables|Default|SetbIsPlaced true))

(fn GetRotatedLocalCELLS
  (bind _lrotcells (LocalVariables|GetLRotCells))
  (Utilities|Array|Clear _lrotcells)
  (for _array_element (Variables|Default|GetLocalCells)
    (bind _cellout (CallFunction|RotateCellAroundPivot _array_element))
    (Utilities|Array|Add _lrotcells _cellout))
  (return (LocalVariables|GetLRotCells)))

(fn RotateSelectAxis
  (params (RotInt :type Integer) (Steps%20Rotated :type Integer))
  (LocalVariables|SetRotation%20Steps Steps%20Rotated)
  (LocalVariables|SetL-PreviewLocalCells (Variables|Default|GetLocalCells))
  (bind _cellsout (CallFunction|ComputeBoardCellsPivot (Variables|Default|GetAnchorCell)))
  (Variables|Default|SetPreviewCells _cellsout)
  (Default|RemoveMapIndex (Variables|Default|GetBoardRef) _cellsout)
  (Utilities|FlowControl|Sequence
    (:then_0
      (switch int RotInt
        (:0
          (LocalVariables|SetLRotXSteps (Variables|Default|GetRotXSteps))
          (Variables|Default|SetRotXSteps (Math|Integer|%(Integer) (+ (Variables|Default|GetRotXSteps) (LocalVariables|GetRotation%20Steps)) 4)))
        (:1
          (LocalVariables|SetLRotYSteps (Variables|Default|GetRotYSteps))
          (Variables|Default|SetRotYSteps (Math|Integer|%(Integer) (+ (Variables|Default|GetRotYSteps) (LocalVariables|GetRotation%20Steps)) 4)))
        (:2
          (LocalVariables|SetLRotZSteps (Variables|Default|GetRotZSteps))
          (Variables|Default|SetRotZSteps (Math|Integer|%(Integer) (+ (Variables|Default|GetRotZSteps) (LocalVariables|GetRotation%20Steps)) 4)))))
    (:then_1
      (bind _cellout (CallFunction|GetRotatedLocalCellsPivoted))
      (Variables|Default|SetLocalCells _cellout)
      (bind _cellsout_2 (CallFunction|ComputeBoardCellsPivot (Variables|Default|GetAnchorCell)))
      (bind _bsafetoplace (Default|CheckCellOccupied (Variables|Default|GetBoardRef) _cellsout_2))
      (if _bsafetoplace
        (bind _output_get (Variables|Default|SetLocalCells _cellout))
        (CallFunction|BuildVisualfromLocalCellsPivot _output_get)
        (bind _world (Default|GridtoWorld (Variables|Default|GetBoardRef) (Variables|Default|GetAnchorCell)))
        (Transformation|SetActorLocation _world false true)
        (bind _cellsout_3 (CallFunction|ComputeBoardCellsPivot (Variables|Default|GetAnchorCell)))
        (bind _output_get_2 (Variables|Default|SetCurrentCells _cellsout_3))
        (CallFunction|AddCellstoSolveArea _output_get_2)
        (for _array_element _output_get_2
          (Default|SetCellOccupied (Variables|Default|GetBoardRef) _array_element))
        ;[0.15 0.15 0.15 0.5] Zero Out For Clean Rotation
        (Variables|Default|SetRotXSteps 0)
        (Variables|Default|SetRotYSteps 0)
        (Variables|Default|SetRotZSteps 0)
        (else
          (Variables|Default|SetLocalCells (LocalVariables|GetL-PreviewLocalCells))
          (Utilities|FlowControl|Sequence
            (:then_0
              (Variables|Default|SetPreviewCells (Variables|Default|GetCurrentCells))
              (switch int RotInt
                (:0
                  (Variables|Default|SetRotXSteps 0))
                (:1
                  (Variables|Default|SetRotYSteps 0))
                (:2
                  (Variables|Default|SetRotZSteps 0))))
            (:then_1
              (bind _cellsout_4 (CallFunction|ComputeBoardCellsPivot (Variables|Default|GetAnchorCell)))
              (CallFunction|AddCellstoSolveArea _cellsout_4))))))))

(fn RotateCellAroundPivot
  (params (CellIn :type Int%20Vector%20Structure))
  (bind (_x _y _z) (Utilities|Struct|BreakIntVector CellIn))
  (bind _pivotlocalcell (Variables|Default|GetPivotLocalCell))
  (bind _pivotlocalcell_2 (Variables|Default|GetPivotLocalCell))
  (bind _pivotlocalcell_3 (Variables|Default|GetPivotLocalCell))
  (bind _pivotlocalcell_4 (Variables|Default|GetPivotLocalCell))
  (bind (_x_2 _y_2 _z_2) (Utilities|Struct|BreakIntVector _pivotlocalcell))
  ;[0.15 0.15 0.15 0.5] Create Relative Cell
  (LocalVariables|SetLRelCell (Utilities|Struct|MakeIntVector (- _x _x_2) (- _y _y_2) (- _z _z_2)))
  (Utilities|FlowControl|Sequence
    (:then_0
      (for _index (range 0 (- (Variables|Default|GetRotXSteps) 1))
        (bind _cellout (CallFunction|Rot90X (LocalVariables|GetLRelCell)))
        (LocalVariables|SetLRelCell (Utilities|Struct|MakeIntVector (+ (.X (Utilities|Struct|BreakIntVector _cellout)) (.x _pivotlocalcell_2)) (+ (.Y (Utilities|Struct|BreakIntVector _cellout)) (.y _pivotlocalcell_2)) (+ (.Z (Utilities|Struct|BreakIntVector _cellout)) (.z _pivotlocalcell_2))))))
    (:then_1
      (for _index_2 (range 0 (- (Variables|Default|GetRotYSteps) 1))
        (bind _cellout_2 (CallFunction|Rot90Y (LocalVariables|GetLRelCell)))
        (LocalVariables|SetLRelCell (Utilities|Struct|MakeIntVector (+ (.X (Utilities|Struct|BreakIntVector _cellout_2)) (.x _pivotlocalcell_4)) (+ (.Y (Utilities|Struct|BreakIntVector _cellout_2)) (.y _pivotlocalcell_4)) (+ (.Z (Utilities|Struct|BreakIntVector _cellout_2)) (.z _pivotlocalcell_4))))))
    (:then_2
      (for _index_3 (range 0 (- (Variables|Default|GetRotZSteps) 1))
        (bind _cellout_3 (CallFunction|Rot90Z (LocalVariables|GetLRelCell)))
        (LocalVariables|SetLRelCell (Utilities|Struct|MakeIntVector (+ (.X (Utilities|Struct|BreakIntVector _cellout_3)) (.x _pivotlocalcell_3)) (+ (.Y (Utilities|Struct|BreakIntVector _cellout_3)) (.y _pivotlocalcell_3)) (+ (.Z (Utilities|Struct|BreakIntVector _cellout_3)) (.z _pivotlocalcell_3))))))
    (:then_3
      (return (LocalVariables|GetLRelCell)))))

(fn RemoveCellsfromArea
  (params (Cells :type Array%20of%20Int%20Vector%20Structures))
  (bind _boardref (Variables|Default|GetBoardRef))
  (bind _cellmap (Variables|/Game/GameBPs/FillTheCubeBPS/BP_FillTheCubeBoard.BP_FillTheCubeBoard_C|GetCellMap _boardref))
  (for _array_element Cells
    (if (.ReturnValue (Utilities|Map|Find _cellmap _array_element))
      (Utilities|Map|Add _cellmap _array_element false))))

(fn AddCellstoSolveArea
  (params (Cells :type Array%20of%20Int%20Vector%20Structures))
  (bind _boardref (Variables|Default|GetBoardRef))
  (bind _cellmap (Variables|/Game/GameBPs/FillTheCubeBPS/BP_FillTheCubeBoard.BP_FillTheCubeBoard_C|GetCellMap _boardref))
  ;[0.15 0.15 0.15 0.5] Get Key if it is in area update to make it true
  (for _array_element Cells
    (if (and (not (.Value (Utilities|Map|Find _cellmap _array_element))) (.ReturnValue (Utilities|Map|Find _cellmap _array_element)))
      (Utilities|Map|Add _cellmap _array_element true))))

(fn SolveZoneOccupied
  (params (Cells :type Array%20of%20Int%20Vector%20Structures))
  ;[0.15 0.15 0.15 0.5] Input = Preview Cells
  ;[0.15 0.15 0.15 0.5] Check To See If Preview Overlaps with any current cells
  (for _array_element Cells
    (if (.Value (Utilities|Map|Find (Variables|/Game/GameBPs/FillTheCubeBPS/BP_FillTheCubeBoard.BP_FillTheCubeBoard_C|GetCellMap (Variables|Default|GetBoardRef)) _array_element))
      (return false)))
  (return true))

(fn Drag
  (params (Direction :type String) (Pos/Negative :type Integer))
  (bind _boardref (Variables|Default|GetBoardRef))
  (Variables|Default|SetbIsPlaced false)
  (Variables|Default|SetbDragging false)
  (bind _output_get (Variables|Default|SetLastValidCell (Variables|Default|GetAnchorCell)))
  (bind _cellsout (CallFunction|ComputeBoardCellsPivot _output_get))
  (Default|RemoveMapIndex (Variables|Default|GetBoardRef) _cellsout)
  (switch string Direction
    (:X
      ;[0.15 0.15 0.15 0.5] Check To See If Cell Can Move To New Spot, Only Checks Solve Zone Cells To Allow For More Movement
      (bind _output_get_2 (Variables|Default|SetAnchorCell (Utilities|Struct|MakeIntVector (+ (.x (Variables|Default|GetAnchorCell)) Pos/Negative) (.y (Variables|Default|GetAnchorCell)) (.z (Variables|Default|GetAnchorCell)))))
      (bind _cellsout_2 (CallFunction|ComputeBoardCellsPivot _output_get_2))
      (bind _output_get_3 (Variables|Default|SetPreviewCells _cellsout_2))
      (bind _bsafetoplace (Default|CheckCellOccupied (Variables|Default|GetBoardRef) _output_get_3))
      (if _bsafetoplace
        ;[0 0.3 0 0.5] True Can Place the piece
        (bind _output_get_4 (Variables|Default|SetCurrentCells (Variables|Default|GetPreviewCells) :!label _label))
        (for _array_element _output_get_4
          (Default|SetCellOccupied (Variables|Default|GetBoardRef) _array_element))
        (bind _world (Default|GridtoWorld _boardref (Variables|Default|GetAnchorCell)))
        (Transformation|SetActorLocation _world false true)
        (bind _gamecomplete (Default|CheckGameComplete _boardref))
        (if _gamecomplete
          (Default|PlayGameOver _boardref _gamecomplete))
        (bind _returnvalue (Actor|GetActorOfClass "/Game/GameBPs/BP_MoveGizmo.BP_MoveGizmo_C"))
        (Transformation|SetActorLocation _returnvalue _world false true)
        (else
          ;[0.3 0 0 0.5] Adds Self Back To Solve Map If It Cannot Move
          (bind _output_get_5 (Variables|Default|SetAnchorCell (Variables|Default|GetLastValidCell) :!label _label_2))
          (bind _cellsout_3 (CallFunction|ComputeBoardCellsPivot _output_get_5))
          (for _array_element_2 _cellsout_3
            (Default|SetCellOccupied (Variables|Default|GetBoardRef) _array_element_2)
            (CallFunction|PlayScalePulse)))))
    (:Y
      (bind _output_get_6 (Variables|Default|SetAnchorCell (Utilities|Struct|MakeIntVector (.x (Variables|Default|GetAnchorCell)) (+ (.y (Variables|Default|GetAnchorCell)) Pos/Negative) (.z (Variables|Default|GetAnchorCell)))))
      (bind _cellsout_4 (CallFunction|ComputeBoardCellsPivot _output_get_6))
      (bind _output_get_7 (Variables|Default|SetPreviewCells _cellsout_4))
      (bind _bsafetoplace_2 (Default|CheckCellOccupied (Variables|Default|GetBoardRef) _output_get_7))
      (if _bsafetoplace_2
        (goto _label)
        (else
          (goto _label_2))))
    (:Z
      (bind _output_get_8 (Variables|Default|SetAnchorCell (Utilities|Struct|MakeIntVector (.x (Variables|Default|GetAnchorCell)) (.y (Variables|Default|GetAnchorCell)) (+ (.z (Variables|Default|GetAnchorCell)) Pos/Negative))))
      (bind _cellsout_5 (CallFunction|ComputeBoardCellsPivot _output_get_8))
      (bind _output_get_9 (Variables|Default|SetPreviewCells _cellsout_5))
      (bind _bsafetoplace_3 (Default|CheckCellOccupied (Variables|Default|GetBoardRef) _output_get_9))
      (if _bsafetoplace_3
        (goto _label)
        (else
          (goto _label_2))))))

(fn PlacePiece
  (bind _hism_cubes (Variables|Default|GetHISM_Cubes))
  (bind _boardref (Variables|Default|GetBoardRef))
  (bind _returnvalue (Rendering|Material|GetMaterial _hism_cubes 0))
  (LocalVariables|SetbCanPlace true)
  (bind _cellsout (CallFunction|ComputeBoardCellsPivot (Variables|Default|GetAnchorCell)))
  (bind _array_element (Utilities|Array|ForEachLoopwithBreak _cellsout :!label _label)
    (:LoopBody
      (if (not (Default|IsinSolveZone (Variables|Default|GetBoardRef) _array_element))
        (LocalVariables|SetbCanPlace false)
        (goto _label Break)))
    (:Completed
      (if (LocalVariables|GetbCanPlace)
        (bind _cellsout_2 (CallFunction|ComputeBoardCellsPivot (Variables|Default|GetAnchorCell)))
        (CallFunction|AddCellstoSolveArea _cellsout_2)
        (for _array_element_2 _cellsout_2
          (bind _world (Default|GridtoWorld _boardref _array_element_2))
          (bind _cell (Default|WorldtoGridSnapped _boardref _world))
          (bind _returnvalue_2 (Game|SpawnActorfromClass "/Game/GameBPs/FillTheCubeBPS/BP_DummyPiece.BP_DummyPiece_C" (Math|Transform|MakeTransform _world "0, 0, 0" "1.000000,1.000000,1.000000") "Undefined" "MultiplyWithRoot" 0 _cell (Variables|Default|GetPiceeID) 0))
          (bind _output_get (Variables|/Game/GameBPs/FillTheCubeBPS/BP_DummyPiece.BP_DummyPiece_C|SetDummLocationVector _returnvalue_2 _cell))
          (Utilities|Map|Add (Variables|/Game/GameBPs/FillTheCubeBPS/BP_FillTheCubeBoard.BP_FillTheCubeBoard_C|GetSolveCellOccupied (Variables|Default|GetBoardRef)) _output_get _returnvalue_2)
          (Utilities|IsValid _returnvalue
            (:Is%20Valid
              (Rendering|Material|SetMaterial (Variables|/Game/GameBPs/FillTheCubeBPS/BP_DummyPiece.BP_DummyPiece_C|GetCubeMesh _returnvalue_2) 0 _returnvalue)
              (Rendering|Material|SetMaterial (Variables|/Game/GameBPs/FillTheCubeBPS/BP_DummyPiece.BP_DummyPiece_C|GetCubeMesh _returnvalue_2) 1 "/Game/Materials/Material_Instances/Black_Outline.Black_Outline"))))
        (return (* (Utilities|Array|Length _cellsout_2) 5))))))