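; Studio actor that renders a thumbnail image for each piece in the level, for either the normal board or the fill board.
; It spawns a preview piece, applies the player's materials, or maps favorite colors to piece IDs.
; A delayed recursive loop rebuilds each shape from DA_PieceLibrary with its own camera framing and captures it to a render target.
; Images go into the board's PieceIDImageMap, then the player controller adds the game widget.
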(event Custom|CreateThumbnails
  (bind _returnvalue (Transformation|GetActorTransform))
  (bind _returnvalue_2 (Transformation|GetActorTransform))
  (bind _piecetocolormap (Variables|Default|GetPieceToColorMap))
  ;[0.15 0.15 0.15 0.5] Create Piece ->
  (Utilities|FlowControl|Sequence
    (:then_0
      (Utilities|IsValid (Variables|Default|GetBoardRef_T)
        (:Is%20Valid
          (ChildActorComponent|SetChildActorClass (Variables|Default|GetChildActor) "/Game/GameBPs/BP_Piece.BP_Piece_C")
          (bind _returnvalue_3 (Game|SpawnActorfromClass "/Game/GameBPs/BP_Piece.BP_Piece_C" (Math|Transform|MakeTransform (.location _returnvalue) "0, 0, 0" "1.000000,1.000000,1.000000") "Undefined" "MultiplyWithRoot" 0 0))
          (Variables|Default|SetPieceRef _returnvalue_3)
          (Default|WorldtoGridSnapped (Variables|/Game/GameBPs/BP_Piece.BP_Piece_C|GetBoardRef (Variables|Default|GetPieceRef)) (.location _returnvalue))
          (Transformation|SetActorLocation (.location _returnvalue) false true)
          (Transformation|SetActorLocation (Variables|Default|GetPieceRef) (.location _returnvalue) false true)
          (Variables|Default|SetLevelPieces (Variables|/Game/GameBPs/BP_BoardManager.BP_BoardManager_C|GetLevelsPieces (Variables|/Game/GameBPs/BP_Piece.BP_Piece_C|GetBoardRef (Variables|Default|GetPieceRef))))
          (bind _asbp_player_controller (Utilities|Casting|CastToBP_PlayerController (Game|GetPlayerController 0)))
          (Utilities|FlowControl|DelayUntilNextTick)
          (Rendering|Material|SetMaterial (Variables|/Game/GameBPs/BP_Piece.BP_Piece_C|GetHISM_Cubes (Variables|Default|GetPieceRef)) 0 (Variables|/Game/PlayerBPs/BP_PlayerController.BP_PlayerController_C|GetPlayersMaterialPref _asbp_player_controller))
          (Rendering|Material|SetMaterial (Variables|/Game/GameBPs/BP_Piece.BP_Piece_C|GetHISM_Cubes (Variables|Default|GetPieceRef)) 1 (Variables|/Game/PlayerBPs/BP_PlayerController.BP_PlayerController_C|GetOutlineColor _asbp_player_controller)))
        (:Is%20Not%20Valid
          (Utilities|IsValid (Variables|Default|GetFillBoardRef)
            (:Is%20Valid
              (ChildActorComponent|SetChildActorClass (Variables|Default|GetChildActor) "/Game/GameBPs/FillTheCubeBPS/BP_FillPieces.BP_FillPieces_C")
              (bind _returnvalue_4 (Game|SpawnActorfromClass "/Game/GameBPs/FillTheCubeBPS/BP_FillPieces.BP_FillPieces_C" (Math|Transform|MakeTransform (.location _returnvalue_2) "0, 0, 0" "1.000000,1.000000,1.000000") "Undefined" "MultiplyWithRoot" 0 0 0))
              (bind _output_get (Variables|Default|SetFillPieceRef _returnvalue_4))
              (Default|WorldtoGridSnapped (Variables|Default|GetFillBoardRef) (.location _returnvalue_2))
              (Transformation|SetActorLocation (.location _returnvalue_2) false true)
              (Transformation|SetActorLocation _output_get (.location _returnvalue_2) false true)
              (Variables|Default|SetLevelPieces (Variables|/Game/GameBPs/FillTheCubeBPS/BP_FillTheCubeBoard.BP_FillTheCubeBoard_C|GetLevelsPieces (Variables|Default|GetFillBoardRef)))
              (bind _asbp_player_controller_2 (Utilities|Casting|CastToBP_PlayerController (Game|GetPlayerController 0)))
              (Utilities|FlowControl|DelayUntilNextTick)
              (Rendering|Material|SetMaterial (Variables|/Game/GameBPs/FillTheCubeBPS/BP_FillPieces.BP_FillPieces_C|GetHISM_Cubes (Variables|Default|GetFillPieceRef)) 0 (Variables|/Game/PlayerBPs/BP_PlayerController.BP_PlayerController_C|GetPlayersMaterialPref _asbp_player_controller_2))
              (Rendering|Material|SetMaterial (Variables|/Game/GameBPs/FillTheCubeBPS/BP_FillPieces.BP_FillPieces_C|GetHISM_Cubes (Variables|Default|GetFillPieceRef)) 1 (Variables|/Game/PlayerBPs/BP_PlayerController.BP_PlayerController_C|GetOutlineColor _asbp_player_controller_2)))))))
    (:then_1
      (Utilities|FlowControl|DelayUntilNextTick)
      (bind _asbp_player_controller_3 (Utilities|Casting|CastToBP_PlayerController (Game|GetPlayerController 0)))
      (Variables|Default|SetSingle%20Color (Variables|/Game/PlayerBPs/BP_PlayerController.BP_PlayerController_C|GetSingle%20Color _asbp_player_controller_3))
      (if (not (Variables|/Game/PlayerBPs/BP_PlayerController.BP_PlayerController_C|GetSingle%20Color _asbp_player_controller_3))
        (for _array_element (.PieceName (Utilities|Struct|BreakF_LevelPieces (Variables|Default|GetLevelPieces)))
          (bind _returnvalue_5 (Utilities|GetDataTableRow "/Game/GameBPs/GamePieces/DA_PieceLibrary.DA_PieceLibrary" _array_element)
            (:then
              (if (not (.ReturnValue (Utilities|Map|Find _piecetocolormap (.PieceID (Utilities|Struct|BreakF_PieceDef _returnvalue_5)))))
                (Utilities|Map|Add _piecetocolormap (.PieceID (Utilities|Struct|BreakF_PieceDef _returnvalue_5)) (Utilities|Array|Get(acopy) (Variables|/Game/PlayerBPs/BP_PlayerController.BP_PlayerController_C|GetListOfMaterialFavorites _asbp_player_controller_3) (Math|Integer|%(Integer) (Utilities|Map|Length (Variables|Default|GetPieceToColorMap)) (Utilities|Array|Length (Variables|/Game/PlayerBPs/BP_PlayerController.BP_PlayerController_C|GetListOfMaterialFavorites _asbp_player_controller_3)))))))))
        (Variables|/Game/PlayerBPs/BP_PlayerController.BP_PlayerController_C|SetIDtoMaterialMap _asbp_player_controller_3 (Variables|Default|GetPieceToColorMap))))
    (:then_2
      (Utilities|IsValid (Variables|Default|GetBoardRef_T)
        (:Is%20Valid
          (CallFunction|BMGenerateScreenShots))
        (:Is%20Not%20Valid
          (CallFunction|FBMCreateScreenshots))))))

(event Custom|FBM_Create%20Screenshots
  (params (Dimension%201 :type Integer))
  (bind _capture (Variables|Default|GetCapture))
  (bind _levelpieces (Variables|Default|GetLevelPieces))
  (bind _springarm (Variables|Default|GetSpringArm))
  (bind _piecename (Utilities|Struct|BreakF_LevelPieces _levelpieces))
  (Variables|Default|SetLoopRoundint Dimension%201)
  (if (> (Variables|Default|GetLoopRoundint) (- (Utilities|Array|Length _piecename) 1))
    (bind _asbp_player_controller (Utilities|Casting|CastToBP_PlayerController (Game|GetPlayerController 0)))
    (Default|AddWidgettoGame _asbp_player_controller 0 (Variables|Default|GetFillBoardRef))
    (else
      (Utilities|FlowControl|DelayUntilNextTick)
      (bind _returnvalue (Utilities|GetDataTableRow "/Game/GameBPs/GamePieces/DA_PieceLibrary.DA_PieceLibrary" (Utilities|Array|Get(acopy) _piecename Dimension%201))
        (:then
          (Variables|Default|SetPieceIDLoop (.PieceID (Utilities|Struct|BreakF_PieceDef _returnvalue)))
          (bind _output_get (Variables|/Game/GameBPs/FillTheCubeBPS/BP_FillPieces.BP_FillPieces_C|SetLocalCells (Variables|Default|GetFillPieceRef) (.Cells (Utilities|Struct|BreakF_PieceDef _returnvalue))))
          (if (Variables|Default|GetSingle%20Color)
            _
            (else
              (Rendering|Material|SetMaterial (Variables|/Game/GameBPs/FillTheCubeBPS/BP_FillPieces.BP_FillPieces_C|GetHISM_Cubes (Variables|Default|GetFillPieceRef)) 0 (.Value (Utilities|Map|Find (Variables|Default|GetPieceToColorMap) (.PieceID (Utilities|Struct|BreakF_PieceDef _returnvalue)))))))
          (Default|BuildVisualfromLocalCellsPivot (Variables|Default|GetFillPieceRef) _output_get)
          ;[0.15 0.15 0.15 0.5] Setting Best Camera angle per piece
          (if (Utilities|Operators|EqualEqual :A (.CameraAngle (Utilities|Struct|BreakF_PieceDef _returnvalue)))
            (Transformation|SetRelativeRotation _springarm (Variables|Default|GetDefaultRotation) false false)
            (else
              (Transformation|SetRelativeRotation _springarm (.CameraAngle (Utilities|Struct|BreakF_PieceDef _returnvalue)) false false)))
          (Variables|/Script/Engine.SceneCaptureComponent2D|SetOrthoWidth _capture (.OrthoWidth (Utilities|Struct|BreakF_PieceDef _returnvalue)))
          (Transformation|SetRelativeLocation _capture (.CameraLocations (Utilities|Struct|BreakF_PieceDef _returnvalue)) false true)
          (Utilities|FlowControl|Delay 0.15)
          (CallFunction|ScreenShotImage))))))

(event Custom|BM_Generate%20ScreenShots
  (params (Dimension%201 :type Integer))
  (bind _levelpieces (Variables|Default|GetLevelPieces))
  (bind _springarm (Variables|Default|GetSpringArm))
  (bind _capture (Variables|Default|GetCapture))
  (bind _piecename (Utilities|Struct|BreakF_LevelPieces _levelpieces))
  (Variables|Default|SetLoopRoundint Dimension%201)
  (if (> (Variables|Default|GetLoopRoundint) (- (Utilities|Array|Length _piecename) 1))
    (bind _asbp_player_controller (Utilities|Casting|CastToBP_PlayerController (Game|GetPlayerController 0)))
    (Default|AddWidgettoGame _asbp_player_controller (Variables|Default|GetBoardRef_T))
    (else
      (Utilities|FlowControl|DelayUntilNextTick)
      (bind _returnvalue (Utilities|GetDataTableRow "/Game/GameBPs/GamePieces/DA_PieceLibrary.DA_PieceLibrary" (Utilities|Array|Get(acopy) _piecename Dimension%201))
        (:then
          (Variables|Default|SetPieceIDLoop (.PieceID (Utilities|Struct|BreakF_PieceDef _returnvalue)))
          (bind _output_get (Variables|/Game/GameBPs/BP_Piece.BP_Piece_C|SetLocalCells (Variables|Default|GetPieceRef) (.Cells (Utilities|Struct|BreakF_PieceDef _returnvalue))))
          (if (Variables|Default|GetSingle%20Color)
            _
            (else
              (Rendering|Material|SetMaterial (Variables|/Game/GameBPs/BP_Piece.BP_Piece_C|GetHISM_Cubes (Variables|Default|GetPieceRef)) 0 (.Value (Utilities|Map|Find (Variables|Default|GetPieceToColorMap) (.PieceID (Utilities|Struct|BreakF_PieceDef _returnvalue)))))))
          (Default|BuildVisualfromLocalCellsPivot (Variables|Default|GetPieceRef) _output_get)
          ;[0.15 0.15 0.15 0.5] Setting Best Camera angle per piece
          (if (Utilities|Operators|EqualEqual :A (.CameraAngle (Utilities|Struct|BreakF_PieceDef _returnvalue)))
            (Transformation|SetRelativeRotation _springarm (Variables|Default|GetDefaultRotation) false false)
            (else
              (Transformation|SetRelativeRotation _springarm (.CameraAngle (Utilities|Struct|BreakF_PieceDef _returnvalue)) false false)))
          (Variables|/Script/Engine.SceneCaptureComponent2D|SetOrthoWidth _capture (.OrthoWidth (Utilities|Struct|BreakF_PieceDef _returnvalue)))
          (Transformation|SetRelativeLocation _capture (.CameraLocations (Utilities|Struct|BreakF_PieceDef _returnvalue)) false true)
          (if (== (Variables|Default|GetLoopRoundint) 0)
            (Utilities|FlowControl|Delay 0.3)
            (else
              (Utilities|FlowControl|Delay 0.15)))
          (CallFunction|ScreenShotImage))))))

(event Custom|ScreenShotImage
  (bind _capture (Variables|Default|GetCapture))
  (bind _boardref_t (Variables|Default|GetBoardRef_T))
  (Utilities|FlowControl|Sequence
    (:then_0
      (bind _returnvalue (Rendering|CreateRenderTarget2D 512 512 "RTF_RGBA8"))
      (bind _output_get (Variables|/Script/Engine.SceneCaptureComponent2D|SetTextureTarget _capture _returnvalue))
      (Rendering|SceneCapture|CaptureScene _capture :!class /Script/Engine.SceneCaptureComponent2D)
      (Utilities|IsValid _output_get
        (:Is%20Valid
          (Utilities|IsValid _boardref_t
            (:Is%20Valid
              (Utilities|Map|Add (Variables|/Game/GameBPs/BP_BoardManager.BP_BoardManager_C|GetPieceIDImageMap _boardref_t) (Variables|Default|GetPieceIDLoop) _output_get))
            (:Is%20Not%20Valid
              (Utilities|Map|Add (Variables|/Game/GameBPs/FillTheCubeBPS/BP_FillTheCubeBoard.BP_FillTheCubeBoard_C|GetPieceIDImageMap (Variables|Default|GetFillBoardRef)) (Variables|Default|GetPieceIDLoop) _output_get))))))
    (:then_1
      (Utilities|IsValid (Variables|Default|GetBoardRef_T)
        (:Is%20Valid
          (CallFunction|BMGenerateScreenShots (+ (Variables|Default|GetLoopRoundint) 1)))
        (:Is%20Not%20Valid
          (CallFunction|FBMCreateScreenshots (+ (Variables|Default|GetLoopRoundint) 1)))))))

(fn ConstructionScript)