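; BP_BoardManager runs the 3D grid board for a cube puzzle level, loading its size, margin and pieces from DA_LevelConfig.
; CreatePuzzle centers the board on the actor and draws the inner solve zone as HISM hologram instances.
; An IntVector-to-bool CellMap tracks solve-cell occupancy for placement and completion checks.
; PlayGameOver spawns the completion effect, saves level stats, shows the game-over widget and hides the move gizmo.
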(event EventBeginPlay
  (bind _solveoccupancy (Variables|Default|GetSolveOccupancy))
  (Utilities|FlowControl|Sequence
    (:then_0
      (bind _asgi_puzzle_game_select (Utilities|Casting|CastToGI_PuzzleGameSelect (Game|GetGameInstance)))
      (bind _returnvalue (Utilities|GetDataTableRow "/Game/GameBPs/GamePieces/DA_LevelConfig.DA_LevelConfig" (.levelname (Variables|/Game/GameBPs/GI_PuzzleGameSelect.GI_PuzzleGameSelect_C|GetLevelSelection _asgi_puzzle_game_select)))
        (:then
          (Variables|Default|SetLevelName (.levelname _returnvalue))
          (Variables|Default|SetLevelsPieces (.levelpieces _returnvalue))
          (Variables|Default|SetPuzzleSizeN (.puzzlesize _returnvalue))
          (Variables|Default|SetMargin (.marginsize _returnvalue))
          (bind _returnvalue_2 (Actor|GetActorOfClass "/Game/GameBPs/BP_ThumbnailStudio.BP_ThumbnailStudio_C"))
          (Default|CreateThumbnails _returnvalue_2)
          (Variables|Default|SetMinimumMoves (Utilities|Array|Length (.PieceID (Utilities|Struct|BreakF_LevelPieces (.levelpieces _returnvalue))))))))
    (:then_1
      (CallFunction|CreatePuzzle))
    (:then_2
      (bind _output_get (Variables|Default|SetSolveCellCount (* (Variables|Default|GetPuzzleSizeN) (Variables|Default|GetPuzzleSizeN) (Variables|Default|GetPuzzleSizeN))))
      (Variables|Default|SetiPuzzleSize _output_get)
      (Utilities|Array|Clear (Variables|Default|GetSolveOccupancy))
      (while (>= (Variables|Default|GetiPuzzleSize) 2)
        (Utilities|Array|Add _solveoccupancy (+ (Utilities|Array|Length _solveoccupancy) 1))
        (bind _result (Math|Integer|DecrementInt (Variables|Default|GetiPuzzleSize))
          (:%20%20
            (Variables|Default|SetiPuzzleSize _result)
            (CallFunction|CreateSolveZoneMap)))))))

(fn ConstructionScript)

(fn GridtoWorld
  (params (Cell :type Int%20Vector%20Structure))
  (return (+ (Variables|Default|GetBoardOrginWorld) (Math|Vector|MakeVector (* (.x Cell) (Variables|Default|GetCellSize)) (* (.y Cell) (Variables|Default|GetCellSize)) (* (.z Cell) (Variables|Default|GetCellSize))))))

(fn WorldtoGridSnapped
  (params (World :type Vector))
  (bind _cellsize (Variables|Default|GetCellSize))
  (return (Class|KismetMathLibrary|FTruncVector (/ (- World (Variables|Default|GetBoardOrginWorld)) (Math|Vector|MakeVector _cellsize _cellsize _cellsize)))))

(fn IsinBounds
  (params (Cell :type Int%20Vector%20Structure))
  (return (Math|Boolean|ANDBoolean (>= (.x Cell) 0) (>= (.y Cell) 0) (>= (.z Cell) 0))))

(fn IsinSolveZone
  (params (Cell :type Int%20Vector%20Structure))
  (bind _x (Utilities|Struct|BreakIntVector Cell))
  (bind _y (Utilities|Struct|BreakIntVector Cell))
  (bind _z (Utilities|Struct|BreakIntVector Cell))
  (return (Math|Boolean|ANDBoolean (and (<= (.x (Variables|Default|GetSolveMin)) _x) (>= (.x (Variables|Default|GetSolveMax)) _x)) (and (<= (.y (Variables|Default|GetSolveMin)) _y) (>= (.y (Variables|Default|GetSolveMax)) _y)) (and (<= (.z (Variables|Default|GetSolveMin)) _z) (>= (.z (Variables|Default|GetSolveMax)) _z)))))

(fn BoardCelltoSolveLocal
  (params (Cell :type Int%20Vector%20Structure))
  (bind _solvemin (Variables|Default|GetSolveMin))
  (return (Utilities|Struct|MakeIntVector (- (.x Cell) (.x _solvemin)) (- (.y Cell) (.y _solvemin)) (- (.z Cell) (.z _solvemin)))))

(fn SolveLocaltoIndex
  (params (Local :type Int%20Vector%20Structure))
  (bind _solvemin (Variables|Default|GetSolveMin))
  (bind _puzzlesizen (Variables|Default|GetPuzzleSizeN))
  ;[0.15 0.15 0.15 0.5] LX/LY/LZ - SolveMin Equation = LX + (LY * N) + (LZ * N * N)
  (return (+ (- (.x Local) (.x _solvemin)) (+ (* (- (.y Local) (.y _solvemin)) _puzzlesizen) (* (- (.z Local) (.z _solvemin)) _puzzlesizen _puzzlesizen)))))

(fn CanPlaceinSolveZone
  (params (Cells :type Array%20of%20Int%20Vector%20Structures))
  (LocalVariables|SetCanPlace true)
  (bind _array_element (Utilities|Array|ForEachLoopwithBreak Cells :!label _label)
    (:LoopBody
      (if (not (CallFunction|IsinSolveZone _array_element))
        (LocalVariables|SetCanPlace false)
        (goto _label Break)))
    (:Completed
      (return (LocalVariables|GetCanPlace)))))

(fn CreateSolveZoneMap
  (bind _solvemin (Variables|Default|GetSolveMin))
  (bind _solvemax (Variables|Default|GetSolveMax))
  (Utilities|Map|Clear (Variables|Default|GetCellMap))
  (for _index (range (.x _solvemin) (.x _solvemax))
    (for _index_2 (range (.y _solvemin) (.y _solvemax))
      (for _index_3 (range (.z _solvemin) (.z _solvemax))
        (Utilities|Map|Add (Variables|Default|GetCellMap) (Utilities|Struct|MakeIntVector _index _index_2 _index_3) false)))))

(fn SetCellOccupied
  (params (Cell :type Int%20Vector%20Structure))
  (bind _cellmap (Variables|Default|GetCellMap))
  (if (.ReturnValue (Utilities|Map|Find _cellmap Cell))
    (Utilities|Map|Add _cellmap Cell true)))

(fn CheckGameComplete
  ;[0.15 0.15 0.15 0.5] Go through all values of Cell Map, if any are false return false
  (bind _values (Utilities|Map|Values (Variables|Default|GetCellMap)))
  (for _array_element _values
    (if (not _array_element)
      (return false)))
  (bind _asbp_player_controller (Utilities|Casting|CastToBP_PlayerController (Game|GetPlayerController 0)))
  (Variables|/Game/PlayerBPs/PlayerHUD/WBP_PlayGameHUD.WBP_PlayGameHUD_C|SetbTimerRunning (Variables|/Game/PlayerBPs/BP_PlayerController.BP_PlayerController_C|GetHUDRef _asbp_player_controller) false)
  (Variables|Default|SetPuzzleTimeTaken (Variables|/Game/PlayerBPs/PlayerHUD/WBP_PlayGameHUD.WBP_PlayGameHUD_C|GetElapsedTime (Variables|/Game/PlayerBPs/BP_PlayerController.BP_PlayerController_C|GetHUDRef _asbp_player_controller)))
  (return true))

(fn CheckCellOccupied
  (params (Cell :type Array%20of%20Int%20Vector%20Structures))
  (for _array_element Cell
    (if (.Value (Utilities|Map|Find (Variables|Default|GetCellMap) _array_element))
      (return false)
      (else
        ;[0.15 0.15 0.15 0.5] Make Sure Move Is Inside The Game Board
        (if (not (Math|Boolean|ANDBoolean (>= (.X (Utilities|Struct|BreakIntVector _array_element)) 0) (<= (.X (Utilities|Struct|BreakIntVector _array_element)) (+ (- (Variables|Default|GetPuzzleSizeN) 1) (* (Variables|Default|GetMargin) 2))) (>= (.Y (Utilities|Struct|BreakIntVector _array_element)) 0) (<= (.Y (Utilities|Struct|BreakIntVector _array_element)) (+ (- (Variables|Default|GetPuzzleSizeN) 1) (* (Variables|Default|GetMargin) 2))) (>= (.Z (Utilities|Struct|BreakIntVector _array_element)) 0) (<= (.Z (Utilities|Struct|BreakIntVector _array_element)) (+ (- (Variables|Default|GetPuzzleSizeN) 1) (* (Variables|Default|GetMargin) 2)))))
          (return false)))))
  (return true))

(fn RemoveMapIndex
  (params (Cells :type Array%20of%20Int%20Vector%20Structures))
  (bind _cellmap (Variables|Default|GetCellMap))
  (for _array_element Cells
    (if (.ReturnValue (Utilities|Map|Find _cellmap _array_element))
      (Utilities|Map|Add _cellmap _array_element false))))

(fn GetImage
  (params (PieceID :type Integer))
  (bind _pieceidimagemap (Variables|Default|GetPieceIDImageMap))
  (bind _value (Utilities|Map|Find _pieceidimagemap PieceID))
  (if (Utilities|Map|Contains _pieceidimagemap PieceID)
    (Utilities|IsValid _value
      (:Is%20Valid
        (return _value)))))

(fn CreatePuzzle
  (Utilities|FlowControl|Sequence
    (:then_0
      ;[0.15 0.15 0.15 0.5] Board/Margin setup -> Set CenterGrid
      (Variables|Default|SetBoardSize (+ (Variables|Default|GetPuzzleSizeN) (* (Variables|Default|GetMargin) 2)))
      (Variables|Default|SetCenterGrid (Class|KismetMathLibrary|ToIntVector(Integer) (/ (- (Variables|Default|GetBoardSize) 1) 2))))
    (:then_1
      ;[0.15 0.15 0.15 0.5] Set SolveMin
      (Variables|Default|SetSolveMin (Class|KismetMathLibrary|ToIntVector(Integer) (Variables|Default|GetMargin)))
      ;[0.15 0.15 0.15 0.5] Set SolveMax
      (Variables|Default|SetSolveMax (Class|KismetMathLibrary|ToIntVector(Integer) (- (+ (Variables|Default|GetMargin) (Variables|Default|GetPuzzleSizeN)) 1)))
      (Variables|Default|SetSolveCenterGrid (Utilities|Struct|MakeIntVector (/ (+ (.x (Variables|Default|GetSolveMin)) (.x (Variables|Default|GetSolveMax))) 2) (/ (+ (.y (Variables|Default|GetSolveMin)) (.y (Variables|Default|GetSolveMax))) 2) (/ (+ (.z (Variables|Default|GetSolveMin)) (.z (Variables|Default|GetSolveMax))) 2))))
    (:then_2
      ;[0.15 0.15 0.15 0.5] Set BoardCenterWorld
      (Variables|Default|SetBoardCenterWorld (Transformation|GetActorLocation))
      (Variables|Default|SetBoardOrginWorld (- (Variables|Default|GetBoardCenterWorld) (Math|Vector|MakeVector (* (.x (Variables|Default|GetCenterGrid)) (Variables|Default|GetCellSize)) (* (.y (Variables|Default|GetCenterGrid)) (Variables|Default|GetCellSize)) (* (.z (Variables|Default|GetCenterGrid)) (Variables|Default|GetCellSize))))))
    (:then_3
      (Components|InstancedStaticMesh|ClearInstances (Variables|Default|GetHISM_SolveHologram))
      (for _index (range (.x (Variables|Default|GetSolveMin)) (.x (Variables|Default|GetSolveMax)))
        (for _index_2 (range (.y (Variables|Default|GetSolveMin)) (.y (Variables|Default|GetSolveMax)))
          (for _index_3 (range (.z (Variables|Default|GetSolveMin)) (.z (Variables|Default|GetSolveMax)))
            (bind _world (CallFunction|GridtoWorld (Utilities|Struct|MakeIntVector _index _index_2 _index_3)))
            (Components|InstancedStaticMesh|AddInstance (Variables|Default|GetHISM_SolveHologram) (Math|Transform|MakeTransform _world "0, 0, 0" (Variables|Default|GetHologramSize)) true)))))))

(fn PlayGameOver
  (params (bGameOver :type Boolean))
  (bind _levelname (Variables|Default|GetLevelName))
  (bind _puzzletimetaken (Variables|Default|GetPuzzleTimeTaken))
  (bind _moves (Variables|Default|GetMoves))
  (if bGameOver
    (bind _returnvalue (Game|SpawnActorfromClass "/Game/GameBPs/BP_GameCompleted.BP_GameCompleted_C" (Math|Transform|MakeTransform "0, 0, 0" "0, 0, 0" "1.000000,1.000000,1.000000") "Undefined" "MultiplyWithRoot" 0 0))
    (Default|PulsedCube _returnvalue (Variables|Default|GetPuzzleSizeN) (Variables|Default|GetMargin))
    (Default|AdjustOpacity _returnvalue)
    (bind _asgi_puzzle_game_select (Utilities|Casting|CastToGI_PuzzleGameSelect (Game|GetGameInstance)))
    (Default|LoadorCreateSave _asgi_puzzle_game_select "PlayersLevelProgress")
    (Default|UpdateLevelStats (Variables|/Game/GameBPs/GI_PuzzleGameSelect.GI_PuzzleGameSelect_C|GetSaveRef _asgi_puzzle_game_select) _levelname true _moves _puzzletimetaken)
    (bind _asbp_player_controller (Utilities|Casting|CastToBP_PlayerController (Game|GetPlayerController 0)))
    (Default|SetUpGameOverWidget _asbp_player_controller _levelname _moves _puzzletimetaken)
    (bind _returnvalue_2 (Actor|GetActorOfClass "/Game/PlayerBPs/BP_OrbitPawn.BP_OrbitPawn_C"))
    (Variables|/Game/PlayerBPs/BP_OrbitPawn.BP_OrbitPawn_C|SetbGameOver? _returnvalue_2 true)
    (Default|TutorialCompleted (Variables|/Game/PlayerBPs/BP_OrbitPawn.BP_OrbitPawn_C|GetSave%20Ref _returnvalue_2))
    (bind _returnvalue_3 (Actor|GetActorOfClass "/Game/GameBPs/BP_MoveGizmo.BP_MoveGizmo_C"))
    (Default|HideGizmo _returnvalue_3 true)))