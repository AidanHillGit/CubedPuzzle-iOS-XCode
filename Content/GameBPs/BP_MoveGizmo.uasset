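; Axis gizmo that moves or rotates puzzle pieces, serving both BP_Piece puzzle mode and Fill the Cube mode.
; BeginPlay detects the mode from the board actor and applies saved guideline and hologram settings.
; Capsule hits or direction indices drive the piece's Drag or RotateSelectAxis by MoveMode, with timeline-pulsed arrows.
; Puzzle mode also updates the HUD's move count and in-zone pieces; construction sets spring-arm lengths.
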(event Custom|HitCapsule
  (params (ComponentInteract :type Object%20Object%20Reference))
  (if (== (Variables|Default|GetGameModeVersion) 0)
    (Utilities|IsValid (Variables|Default|GetPieceRef)
      (:Is%20Valid
        (if (Variables|Default|GetbPieceMoved)
          _
          (else
            (CallFunction|UpdateMoves)))
        (if (Variables|Default|GetbMoveMode)
          ;[0.15 0.15 0.15 0.5] Puzzle Gamemode with BP_Piece
          ;;[0.15 0.15 0.15 0.5] Move Piece Position
          (if (== ComponentInteract (Variables|Default|GetCap_XPos))
            (Default|Drag (Variables|Default|GetPieceRef) "X" 1)
            (CallFunction|PulseArrow (Variables|Default|GetDirArrowXPos))
            (Default|PiecesinZone (Variables|/Game/PlayerBPs/PlayerHUD/WBP_HUDController.WBP_HUDController_C|GetWBP_PlayGameHUD (Variables|Default|GetControlWidgetRef)) :!label _label)
            (elif (== ComponentInteract (Variables|Default|GetCap_XNeg))
              (Default|Drag (Variables|Default|GetPieceRef) "X" -1)
              (CallFunction|PulseArrow (Variables|Default|GetDirArrowXNeg))
              (goto _label)
              (elif (== ComponentInteract (Variables|Default|GetCap_YPos))
                (Default|Drag (Variables|Default|GetPieceRef) "Y" 1)
                (CallFunction|PulseArrow (Variables|Default|GetDirArrowYPos))
                (goto _label)
                (elif (== ComponentInteract (Variables|Default|GetCap_YNeg))
                  (Default|Drag (Variables|Default|GetPieceRef) "Y" -1)
                  (CallFunction|PulseArrow (Variables|Default|GetDirArrowYNeg))
                  (goto _label)
                  (elif (== ComponentInteract (Variables|Default|GetCap_ZPos))
                    (Default|Drag (Variables|Default|GetPieceRef) "Z" 1)
                    (CallFunction|PulseArrow (Variables|Default|GetDirArrowZPos))
                    (goto _label)
                    (elif (== ComponentInteract (Variables|Default|GetCap_ZNeg))
                      (Default|Drag (Variables|Default|GetPieceRef) "Z" -1)
                      (CallFunction|PulseArrow (Variables|Default|GetDirArrowZNeg))
                      (goto _label)))))))
          (elif (== ComponentInteract (Variables|Default|GetCap_XPos))
            (Default|RotateSelectAxis (Variables|Default|GetPieceRef) 2 1)
            (CallFunction|PulseRotArrow (Variables|Default|GetRotArrowXPos))
            (Default|PiecesinZone (Variables|/Game/PlayerBPs/PlayerHUD/WBP_HUDController.WBP_HUDController_C|GetWBP_PlayGameHUD (Variables|Default|GetControlWidgetRef)) :!label _label_2)
            (elif (== ComponentInteract (Variables|Default|GetCap_XNeg))
              (Default|RotateSelectAxis (Variables|Default|GetPieceRef) 2 3)
              (CallFunction|PulseRotArrow (Variables|Default|GetRotArrowXNeg))
              (goto _label_2)
              (elif (== ComponentInteract (Variables|Default|GetCap_YPos))
                (Default|RotateSelectAxis (Variables|Default|GetPieceRef) 0 1)
                (CallFunction|PulseRotArrow (Variables|Default|GetRotArrowYPos))
                (goto _label_2)
                (elif (== ComponentInteract (Variables|Default|GetCap_YNeg))
                  (Default|RotateSelectAxis (Variables|Default|GetPieceRef) 0 3)
                  (CallFunction|PulseRotArrow (Variables|Default|GetRotArrowYNeg))
                  (goto _label_2)
                  (elif (== ComponentInteract (Variables|Default|GetCap_ZPos))
                    (Default|RotateSelectAxis (Variables|Default|GetPieceRef) 1 1)
                    (CallFunction|PulseRotArrow (Variables|Default|GetRotArrowZPos))
                    (goto _label_2)
                    (elif (== ComponentInteract (Variables|Default|GetCap_ZNeg))
                      (Default|RotateSelectAxis (Variables|Default|GetPieceRef) 1 3)
                      (CallFunction|PulseRotArrow (Variables|Default|GetRotArrowZNeg))
                      (goto _label_2))))))))))
    (else
      (Utilities|IsValid (Variables|Default|GetFillPieceRef)
        (:Is%20Valid
          (if (Variables|Default|GetbMoveMode)
            ;[0.15 0.15 0.15 0.5] Gamemode Fill the cube with updated BP_FillPiece
            (if (== ComponentInteract (Variables|Default|GetCap_XPos))
              (Default|Drag (Variables|Default|GetFillPieceRef) "X" 1)
              (CallFunction|PulseArrow (Variables|Default|GetDirArrowXPos))
              (elif (== ComponentInteract (Variables|Default|GetCap_XNeg))
                (Default|Drag (Variables|Default|GetFillPieceRef) "X" -1)
                (CallFunction|PulseArrow (Variables|Default|GetDirArrowXNeg))
                (elif (== ComponentInteract (Variables|Default|GetCap_YPos))
                  (Default|Drag (Variables|Default|GetFillPieceRef) "Y" 1)
                  (CallFunction|PulseArrow (Variables|Default|GetDirArrowYPos))
                  (elif (== ComponentInteract (Variables|Default|GetCap_YNeg))
                    (Default|Drag (Variables|Default|GetFillPieceRef) "Y" -1)
                    (CallFunction|PulseArrow (Variables|Default|GetDirArrowYNeg))
                    (elif (== ComponentInteract (Variables|Default|GetCap_ZPos))
                      (Default|Drag (Variables|Default|GetFillPieceRef) "Z" 1)
                      (CallFunction|PulseArrow (Variables|Default|GetDirArrowZPos))
                      (elif (== ComponentInteract (Variables|Default|GetCap_ZNeg))
                        (Default|Drag (Variables|Default|GetFillPieceRef) "Z" -1)
                        (CallFunction|PulseArrow (Variables|Default|GetDirArrowZNeg))))))))
            (elif (== ComponentInteract (Variables|Default|GetCap_XPos))
              (Default|RotateSelectAxis (Variables|Default|GetFillPieceRef) 2 1)
              (CallFunction|PulseRotArrow (Variables|Default|GetRotArrowXPos))
              (elif (== ComponentInteract (Variables|Default|GetCap_XNeg))
                (Default|RotateSelectAxis (Variables|Default|GetFillPieceRef) 2 3)
                (CallFunction|PulseRotArrow (Variables|Default|GetRotArrowXNeg))
                (elif (== ComponentInteract (Variables|Default|GetCap_YPos))
                  (Default|RotateSelectAxis (Variables|Default|GetFillPieceRef) 0 1)
                  (CallFunction|PulseRotArrow (Variables|Default|GetRotArrowYPos))
                  (elif (== ComponentInteract (Variables|Default|GetCap_YNeg))
                    (Default|RotateSelectAxis (Variables|Default|GetFillPieceRef) 0 3)
                    (CallFunction|PulseRotArrow (Variables|Default|GetRotArrowYNeg))
                    (elif (== ComponentInteract (Variables|Default|GetCap_ZPos))
                      (Default|RotateSelectAxis (Variables|Default|GetFillPieceRef) 1 1)
                      (elif (== ComponentInteract (Variables|Default|GetCap_ZNeg))
                        (Default|RotateSelectAxis (Variables|Default|GetFillPieceRef) 1 3)
                        (CallFunction|PulseRotArrow (Variables|Default|GetRotArrowZNeg))))))))))))))

(event Custom|PreviewDirection
  (params (DirectionIndex :type Integer))
  (bind _bmovemode (Variables|Default|GetbMoveMode))
  (bind _bmovemode_2 (Variables|Default|GetbMoveMode))
  (bind _bmovemode_3 (Variables|Default|GetbMoveMode))
  (bind _bmovemode_4 (Variables|Default|GetbMoveMode))
  (Utilities|FlowControl|Sequence
    (:then_0
      (Development|SetHiddeninGame (Variables|Default|GetDirArrowXPos) true false))
    (:then_1
      (switch int DirectionIndex
        (:0
          (Development|SetHiddeninGame (Variables|Default|GetDirArrowXPos) (not _bmovemode) false)
          (Development|SetHiddeninGame (Variables|Default|GetRotArrowXPos) _bmovemode false))
        (:1
          (Development|SetHiddeninGame (Variables|Default|GetDirArrowXNeg) (not _bmovemode_2) false)
          (Development|SetHiddeninGame (Variables|Default|GetRotArrowXNeg) _bmovemode_2 false))
        (:2
          (Development|SetHiddeninGame (Variables|Default|GetDirArrowYPos) (not _bmovemode_3) false)
          (Development|SetHiddeninGame (Variables|Default|GetRotArrowYPos) _bmovemode_3 false))
        (:3
          (Development|SetHiddeninGame (Variables|Default|GetDirArrowYNeg) (not _bmovemode_4) false)
          (Development|SetHiddeninGame (Variables|Default|GetRotArrowYNeg) _bmovemode_4 false))))))

(event Custom|RestoreVisuals
  ;[0.15 0.15 0.15 0.5] Create Visual based off mode
  (Development|SetHiddeninGame (Variables|Default|GetDirArrowXNeg) (not (stale Custom|SetVisuals _output_get)) false)
  (Development|SetHiddeninGame (Variables|Default|GetRotArrowXPos) (stale Custom|SetVisuals _output_get) false))

(event Custom|MoveOrRotatePiece
  (params (DirectionIndex :type Integer))
  (Utilities|IsValid (Variables|Default|GetPieceRef)
    (:Is%20Valid
      (Utilities|FlowControl|Sequence
        (:then_0
          (switch int DirectionIndex
            (:0
              (if (Variables|Default|GetbMoveMode)
                (Default|Drag (Variables|Default|GetPieceRef) "X" 1)
                (CallFunction|PulseArrow (Variables|Default|GetDirArrowXPos))
                (else
                  (Default|RotateSelectAxis (Variables|Default|GetPieceRef) 2 1)
                  (CallFunction|PulseRotArrow (Variables|Default|GetRotArrowXPos)))))
            (:1
              (if (Variables|Default|GetbMoveMode)
                (Default|Drag (Variables|Default|GetPieceRef) "X" -1)
                (CallFunction|PulseArrow (Variables|Default|GetDirArrowXNeg))
                (else
                  (Default|RotateSelectAxis (Variables|Default|GetPieceRef) 2 3)
                  (CallFunction|PulseRotArrow (Variables|Default|GetRotArrowXNeg)))))
            (:2
              (if (Variables|Default|GetbMoveMode)
                (Default|Drag (Variables|Default|GetPieceRef) "Y" 1)
                (CallFunction|PulseArrow (Variables|Default|GetDirArrowYPos))
                (else
                  (Default|RotateSelectAxis (Variables|Default|GetPieceRef) 0 1)
                  (CallFunction|PulseRotArrow (Variables|Default|GetRotArrowYPos)))))
            (:3
              (if (Variables|Default|GetbMoveMode)
                (Default|Drag (Variables|Default|GetPieceRef) "Y" -1)
                (CallFunction|PulseArrow (Variables|Default|GetDirArrowYNeg))
                (else
                  (Default|RotateSelectAxis (Variables|Default|GetPieceRef) 0 3)
                  (CallFunction|PulseRotArrow (Variables|Default|GetRotArrowYNeg)))))))
        (:then_1
          (Default|PiecesinZone (Variables|/Game/PlayerBPs/PlayerHUD/WBP_HUDController.WBP_HUDController_C|GetWBP_PlayGameHUD (Variables|Default|GetControlWidgetRef))))
        (:then_2
          (CallFunction|UpdateMoves))))
    (:Is%20Not%20Valid
      (switch int DirectionIndex
        (:0
          (if (Variables|Default|GetbMoveMode)
            (Default|Drag (Variables|Default|GetFillPieceRef) "X" 1)
            (CallFunction|PulseArrow (Variables|Default|GetDirArrowXPos))
            (else
              (Default|RotateSelectAxis (Variables|Default|GetFillPieceRef) 2 1)
              (CallFunction|PulseRotArrow (Variables|Default|GetRotArrowXPos)))))
        (:1
          (if (Variables|Default|GetbMoveMode)
            (Default|Drag (Variables|Default|GetFillPieceRef) "X" -1)
            (CallFunction|PulseArrow (Variables|Default|GetDirArrowXNeg))
            (else
              (Default|RotateSelectAxis (Variables|Default|GetFillPieceRef) 2 3)
              (CallFunction|PulseRotArrow (Variables|Default|GetRotArrowXNeg)))))
        (:2
          (if (Variables|Default|GetbMoveMode)
            (Default|Drag (Variables|Default|GetFillPieceRef) "Y" 1)
            (CallFunction|PulseArrow (Variables|Default|GetDirArrowYPos))
            (else
              (Default|RotateSelectAxis (Variables|Default|GetFillPieceRef) 0 1)
              (CallFunction|PulseRotArrow (Variables|Default|GetRotArrowYPos)))))
        (:3
          (if (Variables|Default|GetbMoveMode)
            (Default|Drag (Variables|Default|GetFillPieceRef) "Y" -1)
            (CallFunction|PulseArrow (Variables|Default|GetDirArrowYNeg))
            (else
              (Default|RotateSelectAxis (Variables|Default|GetFillPieceRef) 0 3)
              (CallFunction|PulseRotArrow (Variables|Default|GetRotArrowYNeg)))))))))

(event Custom|SetVisuals
  (params (bMoveMode :type Boolean))
  ;[0.15 0.15 0.15 0.5] Create Visual based off mode
  (bind _output_get (Variables|Default|SetbMoveMode bMoveMode))
  (Development|SetHiddeninGame (Variables|Default|GetDirArrowXNeg) (not _output_get) false)
  (Development|SetHiddeninGame (Variables|Default|GetRotArrowXPos) _output_get false))

(event Custom|PulseArrow
  (params (DirectionalArrowMesh :type Static%20Mesh%20Component%20Object%20Reference))
  ;[0.15 0.15 0.15 0.5] Animation Timelines, Directional Arrow and Pulse Arrow
  (bind _newtrack_0 (Timeline|PulseArrowTimeline PlayFromStart)
    (:Update
      (Transformation|SetRelativeScale3D DirectionalArrowMesh (* (Transformation|GetActorScale3D) (Math|Vector|MakeVector (* _newtrack_0 0.8) (* _newtrack_0 0.8) (* _newtrack_0 0.8)))))
    (:Finished
      (Transformation|SetRelativeScale3D DirectionalArrowMesh "0.800000,0.800000,0.800000"))))

(event Custom|PulseRotArrow
  (params (RotArrowZNeg :type Static%20Mesh%20Component%20Object%20Reference))
  ;[0.15 0.15 0.15 0.5] Animation Timelines, Directional Arrow and Pulse Arrow
  (bind _newtrack_0 (Timeline|Timeline PlayFromStart)
    (:Update
      (Transformation|SetRelativeScale3D RotArrowZNeg (* (Transformation|GetActorScale3D) (Math|Vector|MakeVector (* _newtrack_0 0.25) (* _newtrack_0 0.25) (* _newtrack_0 0.25)))))
    (:Finished
      (Transformation|SetRelativeScale3D RotArrowZNeg "0.250000,0.250000,0.250000"))))

(event Custom|HideGizmo
  (params (Condition :type Boolean))
  ;[0.15 0.15 0.15 0.5] Create Visual based off mode
  (if Condition
    (Collision|SetCollisionEnabled (Variables|Default|GetCap_XPos) "NoCollision")
    (Rendering|SetActorHiddenInGame true)
    (else
      (Collision|SetCollisionEnabled (Variables|Default|GetCap_XPos) (Variables|Default|GetCollisionPresets))
      (Rendering|SetActorHiddenInGame false))))

(event Custom|HideGuidelines
  (params (Hidden? :type Boolean))
  ;[0.15 0.15 0.15 0.5] Event To Toggle Hide Game Objects
  (Development|SetHiddeninGame (Variables|Default|GetGuideGreen) (not Hidden?) false))

(event Custom|SetArrowMeshColor
  (bind _asgi_puzzle_game_select (Utilities|Casting|CastToGI_PuzzleGameSelect (Game|GetGameInstance)))
  (CallFunction|HideGuidelines (Variables|/Game/GameBPs/GI_PuzzleGameSelect.GI_PuzzleGameSelect_C|GetGuide%20Lines _asgi_puzzle_game_select))
  (Utilities|IsValid (Variables|/Game/PlayerBPs/SaveGame/SG_PlayerProgress.SG_PlayerProgress_C|GetHologramMaterial (Variables|/Game/GameBPs/GI_PuzzleGameSelect.GI_PuzzleGameSelect_C|GetSaveRef _asgi_puzzle_game_select))
    (:Is%20Valid
      (Rendering|Material|SetMaterial (Variables|Default|GetRotArrowXNeg) 0 (Variables|/Game/PlayerBPs/SaveGame/SG_PlayerProgress.SG_PlayerProgress_C|GetHologramMaterial (Variables|/Game/GameBPs/GI_PuzzleGameSelect.GI_PuzzleGameSelect_C|GetSaveRef _asgi_puzzle_game_select))))
    (:Is%20Not%20Valid
      (Default|SaveHologramColor (Variables|/Game/GameBPs/GI_PuzzleGameSelect.GI_PuzzleGameSelect_C|GetSaveRef _asgi_puzzle_game_select) (Variables|/Game/PlayerBPs/SaveGame/SG_PlayerProgress.SG_PlayerProgress_C|GetHologramColor (Variables|/Game/GameBPs/GI_PuzzleGameSelect.GI_PuzzleGameSelect_C|GetSaveRef _asgi_puzzle_game_select)))
      (Rendering|Material|SetMaterial (Variables|Default|GetRotArrowXNeg) 0 (Variables|/Game/PlayerBPs/SaveGame/SG_PlayerProgress.SG_PlayerProgress_C|GetHologramMaterial (Variables|/Game/GameBPs/GI_PuzzleGameSelect.GI_PuzzleGameSelect_C|GetSaveRef _asgi_puzzle_game_select))))))

(event Custom|UpdatePiece
  (params (Condition :type Boolean))
  (bind _pieceref (Variables|Default|GetPieceRef))
  (bind _hism_cubes (Variables|/Game/GameBPs/BP_Piece.BP_Piece_C|GetHISM_Cubes _pieceref))
  (Utilities|IsValid _pieceref
    (:Is%20Valid
      (if Condition
        (Rendering|Material|SetMaterial _hism_cubes 0 "/Game/Materials/Material/SThr_WhiteMat.SThr_WhiteMat")
        (Rendering|Material|SetMaterial _hism_cubes 1 "/Game/Materials/Material/SThr_BlackMat1.SThr_BlackMat1")
        (else
          (Rendering|Material|SetMaterial _hism_cubes 0 "/Game/Materials/Material/SolidWhite_MI.SolidWhite_MI")
          (Rendering|Material|SetMaterial _hism_cubes 1 "/Game/Materials/Material/SolidBlack_MI.SolidBlack_MI"))))))

(event Custom|UpdateMoves
  (bind _pieceref (Variables|Default|GetPieceRef))
  ;[0.15 0.15 0.15 0.5] Call On Puzzle Mode To Update The Board On Movement
  (if (not (Variables|Default|GetbPieceMoved))
    (Utilities|IsValid _pieceref
      (:Is%20Valid
        (Variables|Default|SetbPieceMoved true)
        (bind _result (Math|Integer|IncrementInt (Variables|/Game/GameBPs/BP_BoardManager.BP_BoardManager_C|GetMoves (Variables|/Game/GameBPs/BP_Piece.BP_Piece_C|GetBoardRef _pieceref)))
          (:%20%20
            (Default|UpdateMovesText (Variables|/Game/PlayerBPs/PlayerHUD/WBP_HUDController.WBP_HUDController_C|GetWBP_PlayGameHUD (Variables|Default|GetControlWidgetRef)) _result)))))))

(event EventBeginPlay
  ;[0.15 0.15 0.15 0.5] Get Game Mode, and set collision presets
  (Utilities|FlowControl|Sequence
    (:then_0
      (Variables|Default|SetCollisionPresets (Collision|GetCollisionEnabled (Variables|Default|GetCap_XPos)))
      (CallFunction|SetArrowMeshColor)
      (bind _returnvalue (Actor|GetActorOfClass "/Game/GameBPs/BP_BoardManager.BP_BoardManager_C"))
      (Utilities|IsValid _returnvalue
        (:Is%20Valid
          (Variables|Default|SetGameModeVersion 0))
        (:Is%20Not%20Valid
          (bind _returnvalue_2 (Actor|GetActorOfClass "/Game/GameBPs/FillTheCubeBPS/BP_FillTheCubeBoard.BP_FillTheCubeBoard_C"))
          (Utilities|IsValid _returnvalue_2
            (:Is%20Valid
              (Variables|Default|SetGameModeVersion 1))))))
    (:then_1
      (Collision|SetCollisionEnabled (Variables|Default|GetCap_XPos) "NoCollision"))))

(fn ConstructionScript
  (bind _springarmlength (Variables|Default|GetSpringArmLength))
  (Variables|/Script/Engine.SpringArmComponent|SetTargetArmLength (Variables|Default|GetSpringArmX) _springarmlength)
  (Variables|/Script/Engine.SpringArmComponent|SetTargetArmLength (Variables|Default|GetSpringArmY) _springarmlength)
  (Variables|/Script/Engine.SpringArmComponent|SetTargetArmLength (Variables|Default|GetSpringArmZ) _springarmlength)
  (Variables|/Script/Engine.SpringArmComponent|SetTargetArmLength (Variables|Default|GetSpringArmX1) _springarmlength)
  (Variables|/Script/Engine.SpringArmComponent|SetTargetArmLength (Variables|Default|GetSpringArmY1) _springarmlength)
  (Variables|/Script/Engine.SpringArmComponent|SetTargetArmLength (Variables|Default|GetSpringArmZ1) _springarmlength))